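; Game instance Blueprint that handles restarting the current level after death.
; Its Restart event checks the Dead flag, then clears it and reopens the current level by name, or prints a refusal message if the flag is unset.
; PickupHealth, PickupItem and PickupShield are empty stubs that always return false.
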(event `/Game/Characters/Player/Blueprints/CharacterInterface.Restart`
  (if (`self.Dead?`)
    (set `self.Dead?` false)
    (`KismetSystemLibrary.PrintString` "m8")
    (bind _returnvalue (`GameplayStatics.GetCurrentLevelName` true))
    (`GameplayStatics.OpenLevel` (`KismetStringLibrary.Conv_StringToName` _returnvalue))
    (else
      (`KismetSystemLibrary.PrintString` "Only Restart, When Dead"))))

(fn `PickupHealth`
  (params (BaseHealth :type "Float (double-precision)"))
  (returns (Success :type Boolean))
  (return false))

(fn `PickupItem`
  (params (PickupType :type "/Game/Characters/Player/Blueprints/Inventory/PickupType Enum" :default "NewEnumerator0") (AmmoType :type "/Game/Characters/Player/Blueprints/Inventory/AmmoType Enum" :default "NewEnumerator0") (Count :type Integer) (WeaponClass :type "Actor Class Reference"))
  (returns (Success :type Boolean))
  (return false))

(fn `PickupShield`
  (params (BaseShield :type "Float (double-precision)"))
  (returns (Success :type Boolean))
  (return false))