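; Game mode that runs the level loop: spawning, player lives, game over, currency and checkpoint saves.
; BeginPlay always starts a new game, placing pickups and data-table enemies on shuffled, type-matched spawn points, then spawning the player and HUD and saving.
; Checkpoints save player stats, enemies, currency, lives and level to a slot.
; Death costs a life, then reloads that save (or starts fresh) and re-saves, or shows GameOver at zero.
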(event `self.ReceiveBeginPlay`
  (`|ExecutionSequence`
    (:`then_0`
      (`self.BindEvents`)
      (`KismetSystemLibrary.PrintString` "StartingGame")
      (`self.DoesSaveExist`
        (:`True`
          ;[1 0 0] NO LOAD GAME
          (`KismetSystemLibrary.PrintString` "Save Exists, Loading Preview Game"))
        (:`False`
          (`KismetSystemLibrary.PrintString` "Save does not exist, Starting new game")))
      (`self.NewGame`))))

(event `GameOver`
  (bind _returnvalue (`|CreateWidget` "/Game/UI/GameOver.GameOver_C"))
  (`UserWidget.AddToViewport` _returnvalue 0))

(event `NewGame`
  (`self.SpawnPickups`)
  (`self.SpawnEnemies`)
  (`self.SpawnPlayer` (`self.GetLevelStart`))
  (`/Engine/EditorBlueprintResources/StandardMacros.DoOnce` false
    (:`Completed`
      (`self.SaveGame` null))))

(event `OnPlayerDeath`
  (`Widget.RemoveFromParent` (`self.PlayerHUD`))
  (set `self.CharToDelete` (`self.PlayerCharacter`))
  (bind _asmy_game_instance (cast `/Game/Base/Blueprints/Gamemode/MyGameInstance` (`GameplayStatics.GetGameInstance`)))
  (bind _output_get (set `/Game/Base/Blueprints/Gamemode/MyGameInstance.Lives` (- (`/Game/Base/Blueprints/Gamemode/MyGameInstance.Lives` _asmy_game_instance) 1) _asmy_game_instance))
  (if (<= _output_get 0)
    (`self.GameOver`)
    (else
      (`self.DoesSaveExist`
        (:`True`
          (`self.LoadGame`))
        (:`False`
          (`self.NewGame`)))
      (`self.DestroyIfValid` (`self.CharToDelete`)
        (:`Out`
          (`self.SaveGame` (`self.LastCheckpoint`)))))))

(event `OnCheckPointReached`
  (params (Checkpoint :type "/Game/Base/Blueprints/Gamemode/CheckPoint Object Reference"))
  (set `self.LastCheckpoint` Checkpoint)
  (bind _success (`self.SaveGame` Checkpoint))
  (if _success
    (`KismetSystemLibrary.PrintString` "Saved Game" true false (struct :`R` 0.018076 :`G` 1.0 :`A` 1.0) 5.0)
    (else
      (`KismetSystemLibrary.PrintString` "Failed to save game!" true true (struct :`R` 1.0 :`B` 0.02529 :`A` 1.0) 5.0))))

(fn `BindEvents`
  ;[1 1 1] Checkpoints
  (bind _outactors (`GameplayStatics.GetAllActorsOfClass` "/Game/Base/Blueprints/Gamemode/CheckPoint.CheckPoint_C"))
  (add `/Game/Base/Blueprints/Gamemode/CheckPoint.CheckPointReached` _outactors (`|CreateDelegate` :!event `OnCheckPointReached`)))

(fn `Call Ship`
  ;[1 1 1] Store a Reference and utilise 'Call Ship Event'
  (bind _outactors (`GameplayStatics.GetAllActorsOfClass` "/Game/Weapons/Blueprints/Environmental/BP_Ship.BP_Ship_C"))
  (set `self.BP_ShipRef` (`|GetArrayItem` _outactors))
  (`/Game/Weapons/Blueprints/Environmental/BP_Ship.ActivateShip` (`self.BP_ShipRef`)))

(fn `ChangeCurrency`
  (params (Amount :type Integer))
  (bind _playercharacter (`self.PlayerCharacter`))
  (bind _ui_widget (`/Game/Characters/Player/Blueprints/BP_PlayerCharacter.UI_Widget` _playercharacter))
  (bind _asmy_game_instance (cast `/Game/Base/Blueprints/Gamemode/MyGameInstance` (`GameplayStatics.GetGameInstance`)))
  (bind _output_get (set `/Game/Base/Blueprints/Gamemode/MyGameInstance.Currency` (+ (`/Game/Base/Blueprints/Gamemode/MyGameInstance.Currency` _asmy_game_instance) Amount) _asmy_game_instance))
  (`/Engine/EditorBlueprintResources/StandardMacros.IsValid` _playercharacter
    (:`Is Valid`
      (`/Engine/EditorBlueprintResources/StandardMacros.IsValid` _ui_widget
        (:`Is Valid`
          (`/Game/Characters/Player/Blueprints/DevHUD.UpdateCurrency` _ui_widget _output_get))))))

(fn `GetCurrency`
  (returns (Currency :type Integer))
  (bind _asmy_game_instance (cast `/Game/Base/Blueprints/Gamemode/MyGameInstance` (`GameplayStatics.GetGameInstance`))
    (:`then`
      (return (`/Game/Base/Blueprints/Gamemode/MyGameInstance.Currency` _asmy_game_instance)))
    (:`CastFailed`
      (return 0))))

(fn `GetLevelStart`
  (returns (SpawnTransform :type "Transform Structure"))
  (bind _outactors (`GameplayStatics.GetAllActorsOfClass` "/Game/Base/Blueprints/Gamemode/LevelStart.LevelStart_C"))
  (if (< (`KismetArrayLibrary.Array_Length` _outactors) 1)
    (`KismetSystemLibrary.PrintString` "Error No LevelStarts Present in Level" true true (struct :`R` 1.0 :`B` 0.012401 :`A` 1.0) 10.0)
    (return)
    (else
      (return (`self.GetTransform` (`|GetArrayItem` _outactors))))))

(fn `LoadGame`
  (locals (L_LoadedSave :type "/Game/Base/Blueprints/Gamemode/MySaveGame Object Reference"))
  (bind _returnvalue (`GameplayStatics.LoadGameFromSlot` (`self.SaveSlot`)))
  (bind _asmy_save_game (cast `/Game/Base/Blueprints/Gamemode/MySaveGame` _returnvalue))
  (set `local.L_LoadedSave` _asmy_save_game)
  (bind _returnvalue_2 (`GameplayStatics.GetCurrentLevelName` true))
  (bind _level (`/Game/Base/Blueprints/Gamemode/MySaveGame.Level` _asmy_save_game))
  ;[1 1 1] Check if Player is on correct level
  (if (== (`KismetStringLibrary.Conv_StringToName` _returnvalue_2) _level)
    (`|ExecutionSequence`
      (:`then_0`
        (`|ExecutionSequence`
          (:`then_0`
            ;[1 1 1] Spawn Player
            (`self.SpawnPlayer` (`KismetMathLibrary.Conv_VectorToTransform` (`/Game/Base/Blueprints/Gamemode/MySaveGame.CheckpointLocation` (`local.L_LoadedSave`))) (`/Game/Base/Blueprints/Gamemode/MySaveGame.PlayerStats` (`local.L_LoadedSave`))))
          (:`then_1`
            ;[1 1 1] Spawn Enemies
            ;;[1 1 1] Destroy already existing enemies
            (bind _outactors (`GameplayStatics.GetAllActorsOfClass` "/Game/Characters/Enemies/Blueprints/Classes/EP_Parent.EP_Parent_C"))
            (for _array_element _outactors
              (`self.K2_DestroyActor` _array_element))
            ;;[1 1 1] Spawn Enemies from save data
            (for _array_element_2 (`/Game/Base/Blueprints/Gamemode/MySaveGame.Enemys` (`local.L_LoadedSave`))
              (bind (_enemyclass _health _actortransform) (break `/Game/Base/Blueprints/Gamemode/EnemyStats` _array_element_2))
              (`AIBlueprintHelperLibrary.SpawnAIFromClass` _enemyclass "/Game/Characters/Enemies/Blueprints/BehaviourTrees/BT_Ranged.BT_Ranged" (.location _actortransform) (.rotation _actortransform))))))
      (:`then_1`
        ;[1 1 1] Load Instance Vars
        (bind _asmy_game_instance (cast `/Game/Base/Blueprints/Gamemode/MyGameInstance` (`GameplayStatics.GetGameInstance`)))
        (set `/Game/Base/Blueprints/Gamemode/MyGameInstance.Currency` (`/Game/Base/Blueprints/Gamemode/MySaveGame.Currency` (`local.L_LoadedSave`)) _asmy_game_instance)))
    (else
      ;[1 1 1] Attempt to load correct level
      (`KismetSystemLibrary.PrintString` "Error, wrong level loaded for save data, attempting to switch" true true (struct :`R` 1.0 :`A` 1.0) 5.0)
      (`GameplayStatics.OpenLevel` _level))))

(fn `SaveGame`
  (params (CheckPoint :type "/Game/Base/Blueprints/Gamemode/CheckPoint Object Reference"))
  (returns (Success :type Boolean))
  (locals (L_SaveGame :type "/Game/Base/Blueprints/Gamemode/MySaveGame Object Reference") (L_EnemyStats :type "Array of /Game/Base/Blueprints/Gamemode/EnemyStats Structure"))
  (bind _outactors (`GameplayStatics.GetAllActorsOfClass` "/Game/Base/Blueprints/Gamemode/LevelStart.LevelStart_C"))
  (`|ExecutionSequence`
    (:`then_0`
      ;[1 1 1] Store EnemyData
      (bind _outactors_2 (`GameplayStatics.GetAllActorsOfClass` "/Game/Characters/Enemies/Blueprints/Classes/EP_Parent.EP_Parent_C"))
      (`KismetArrayLibrary.Array_Clear` (`local.L_EnemyStats`))
      (for _array_element _outactors_2
        (`KismetArrayLibrary.Array_Add` (`local.L_EnemyStats`) (make `/Game/Base/Blueprints/Gamemode/EnemyStats` (`GameplayStatics.GetObjectClass` _array_element) (`/Game/Characters/Enemies/Blueprints/Classes/EP_Parent.TotalHP` _array_element) (`self.GetTransform` _array_element) "/Game/Characters/Enemies/Blueprints/BehaviourTrees/BT_Ranged.BT_Ranged"))))
    (:`then_1`
      ;[1 1 1] Create Save Game
      (bind _returnvalue (`GameplayStatics.CreateSaveGameObject` "/Game/Base/Blueprints/Gamemode/MySaveGame.MySaveGame_C"))
      (set `local.L_SaveGame` _returnvalue))
    (:`then_2`
      ;[1 1 1] Set Savegame Variables
      (bind _asbp_player_character (cast `/Game/Characters/Player/Blueprints/BP_PlayerCharacter` (`Controller.K2_GetPawn` (`GameplayStatics.GetPlayerController` 0))))
      (set `/Game/Base/Blueprints/Gamemode/MySaveGame.PlayerStats` (`/Game/Characters/Player/Blueprints/BP_PlayerCharacter.GetPlayerStats` _asbp_player_character) (`local.L_SaveGame`))
      (`|ExecutionSequence`
        (:`then_0`
          (if (`KismetSystemLibrary.IsValid` CheckPoint)
            (set `/Game/Base/Blueprints/Gamemode/MySaveGame.CheckpointLocation` (`self.K2_GetActorLocation` CheckPoint) (`local.L_SaveGame`))
            (else
              (set `/Game/Base/Blueprints/Gamemode/MySaveGame.CheckpointLocation` (`self.K2_GetActorLocation` (`|GetArrayItem` _outactors)) (`local.L_SaveGame`)))))
        (:`then_1`
          (bind _returnvalue_2 (`GameplayStatics.GetCurrentLevelName` true))
          (set `/Game/Base/Blueprints/Gamemode/MySaveGame.Level` (`KismetStringLibrary.Conv_StringToName` _returnvalue_2) (`local.L_SaveGame`))
          (set `/Game/Base/Blueprints/Gamemode/MySaveGame.Enemys` (`local.L_EnemyStats`) (`local.L_SaveGame`))
          (set `/Game/Base/Blueprints/Gamemode/MySaveGame.Currency` (`self.GetCurrency`) (`local.L_SaveGame`))
          (bind _asmy_game_instance (cast `/Game/Base/Blueprints/Gamemode/MyGameInstance` (`GameplayStatics.GetGameInstance`)))
          (set `/Game/Base/Blueprints/Gamemode/MySaveGame.Lives` (`/Game/Base/Blueprints/Gamemode/MyGameInstance.Lives` _asmy_game_instance) (`local.L_SaveGame`)))))
    (:`then_3`
      ;[1 1 1] Save to Slot
      (bind _returnvalue_3 (`GameplayStatics.SaveGameToSlot` (`local.L_SaveGame`) (`self.SaveSlot`)))
      (return _returnvalue_3))))

(fn `SetGameInstancesVariables`
  (bind _asmy_game_instance (cast `/Game/Base/Blueprints/Gamemode/MyGameInstance` (`GameplayStatics.GetGameInstance`)))
  (set `/Game/Base/Blueprints/Gamemode/MyGameInstance.Lives` (`self.DefaultLives`) _asmy_game_instance))

(fn `SpawnEnemies`
  (locals (L_SpawnPoints :type "Array of /Game/Base/Blueprints/ParentSpawnPoint Object Reference") (L_FilteredSpawnPoints :type "Array of /Game/Base/Blueprints/ParentSpawnPoint Object Reference"))
  (bind _output (`|GetArrayItem` (`local.L_FilteredSpawnPoints`)))
  (bind (_returnvalue_location _returnvalue_rotation) (`KismetMathLibrary.BreakTransform` (`self.GetTransform` _output)))
  (bind _outactors (`GameplayStatics.GetAllActorsOfClass` "/Game/Base/Blueprints/ParentSpawnPoint.ParentSpawnPoint_C"))
  (set `local.L_SpawnPoints` _outactors)
  (bind _outrownames (`DataTableFunctionLibrary.GetDataTableRowNames` "/Game/Base/Blueprints/Gamemode/DataTableEnemySpawn.DataTableEnemySpawn"))
  (for _array_element _outrownames
    (bind _returnvalue (`|GetDataTableRow` "/Game/Base/Blueprints/Gamemode/DataTableEnemySpawn.DataTableEnemySpawn" _array_element)
      (:`then`
        (`KismetArrayLibrary.Array_Clear` (`local.L_FilteredSpawnPoints`))
        (`|ExecutionSequence`
          (:`then_0`
            (for _array_element_2 (`local.L_SpawnPoints`)
              (bind (_spawnname _spawntype _spawnclass _behaviortree _count) (break `/Game/Base/Blueprints/Gamemode/EnemySpawnInfo` _returnvalue))
              (if (`|EnumEquality` (`/Game/Base/Blueprints/ParentSpawnPoint.SpawnType` _array_element_2) _spawntype)
                (`KismetArrayLibrary.Array_Add` (`local.L_FilteredSpawnPoints`) _array_element_2))))
          (:`then_1`
            (`KismetArrayLibrary.Array_Shuffle` (`local.L_FilteredSpawnPoints`)))
          (:`then_2`
            (for _ (range 1 (+ _count 1))
              (if (<= (`KismetArrayLibrary.Array_Length` (`local.L_FilteredSpawnPoints`)) 0)
                (`/Engine/EditorBlueprintResources/StandardMacros.DoOnce` false
                  (:`Completed`
                    (`KismetSystemLibrary.PrintString` "Warning, not enough spawn locations present to spawn all enemies!" true true (struct :`R` 1.0 :`G` 0.248857 :`A` 1.0))))
                (else
                  (`AIBlueprintHelperLibrary.SpawnAIFromClass` _spawnclass _behaviortree _returnvalue_location _returnvalue_rotation)
                  (`KismetArrayLibrary.Array_RemoveItem` (`local.L_FilteredSpawnPoints`) _output)
                  (`KismetArrayLibrary.Array_RemoveItem` (`local.L_SpawnPoints`) _output))))))))))

(fn `SpawnPickups`
  (locals (L_SpawnPoints :type "Array of /Game/Base/Blueprints/ParentSpawnPoint Object Reference") (L_FilteredSpawnPoints :type "Array of /Game/Base/Blueprints/ParentSpawnPoint Object Reference"))
  (bind _output (`|GetArrayItem` (`local.L_FilteredSpawnPoints`)))
  (bind _outactors (`GameplayStatics.GetAllActorsOfClass` "/Game/Base/Blueprints/ParentSpawnPoint.ParentSpawnPoint_C"))
  (set `local.L_SpawnPoints` _outactors)
  (for _array_element (`self.SpawnInfo`)
    (`KismetArrayLibrary.Array_Clear` (`local.L_FilteredSpawnPoints`))
    (`|ExecutionSequence`
      (:`then_0`
        (for _array_element_2 (`local.L_SpawnPoints`)
          (bind (_spawnname _spawntype _minamount _maxamount _pickup) (break `/Game/Base/Blueprints/Gamemode/SpawnInfo` _array_element))
          (if (`|EnumEquality` (`/Game/Base/Blueprints/ParentSpawnPoint.SpawnType` _array_element_2) _spawntype)
            (`KismetArrayLibrary.Array_Add` (`local.L_FilteredSpawnPoints`) _array_element_2))))
      (:`then_1`
        (`KismetArrayLibrary.Array_Shuffle` (`local.L_FilteredSpawnPoints`)))
      (:`then_2`
        (for _ (range (+ (`KismetMathLibrary.RandomIntegerInRange` _minamount _maxamount) 1))
          (if (<= (`KismetArrayLibrary.Array_Length` (`local.L_FilteredSpawnPoints`)) 0)
            (`/Engine/EditorBlueprintResources/StandardMacros.DoOnce` false
              (:`Completed`
                (`KismetSystemLibrary.PrintString` "Warning, not enough spawn locations present to spawn all items!" true true (struct :`R` 1.0 :`G` 0.248857 :`A` 1.0))
                (break)))
            (else
              (`|SpawnActorFromClass` "/Game/Base/Blueprints/Pickups/BP_Pickup.BP_Pickup_C" (`self.GetTransform` _output) "Undefined" "OverrideRootScale" null _pickup null)
              (`KismetArrayLibrary.Array_RemoveItem` (`local.L_FilteredSpawnPoints`) _output)
              (`KismetArrayLibrary.Array_RemoveItem` (`local.L_SpawnPoints`) _output))))))))

(fn `SpawnPlayer`
  (params (`Spawn Transform` :type "Transform Structure") (PlayerStats :type "/Game/Base/Blueprints/Gamemode/PlayerStats Structure"))
  (returns (PlayerChar :type "/Game/Characters/Player/Blueprints/BP_PlayerCharacter Object Reference"))
  (locals (L_SpawnTransform :type "Transform Structure") (L_PlayerStats :type "/Game/Base/Blueprints/Gamemode/PlayerStats Structure"))
  (bind _playercharacter (`self.PlayerCharacter`))
  (bind (_health _shields _stamina _ammobullets _ammolasers _weapons _ammogrenade) (break `/Game/Base/Blueprints/Gamemode/PlayerStats` (`local.L_PlayerStats`)))
  (bind _bp_inventory (`/Game/Characters/Player/Blueprints/BP_PlayerCharacter.BP_Inventory` _playercharacter))
  (set `local.L_SpawnTransform` `Spawn Transform`)
  (set `local.L_PlayerStats` PlayerStats)
  ;[1 1 1] Spawn and Set player char
  (bind _returnvalue (`|SpawnActorFromClass` "/Game/Characters/Player/Blueprints/BP_PlayerCharacter.BP_PlayerCharacter_C" (`local.L_SpawnTransform`) "AdjustIfPossibleButAlwaysSpawn" "OverrideRootScale" null null))
  (bind _output_get (set `self.PlayerCharacter` _returnvalue))
  (`|ExecutionSequence`
    (:`then_0`
      ;[1 1 1] Spawn Widget
      (bind _returnvalue_2 (`|CreateWidget` "/Game/UI/PlayerHUD.PlayerHUD_C" (`GameplayStatics.GetPlayerController` 0)))
      (bind _output_get_2 (set `self.PlayerHUD` _returnvalue_2))
      (`UserWidget.AddToViewport` _output_get_2 0)
      (`/Game/UI/PlayerHUD.Init` (`self.PlayerHUD`) (`self.PlayerCharacter`)))
    (:`then_1`
      ;[1 1 1] Bind Events
      (add `/Game/Characters/Player/Blueprints/BP_PlayerCharacter.PlayerDeath` (`self.PlayerCharacter`) (`|CreateDelegate` :!event `OnPlayerDeath`)))
    (:`then_2`
      ;[1 1 1] Set Stats
      (set `/Game/Characters/Player/Blueprints/BP_PlayerCharacter.Health` _health _playercharacter)
      (set `/Game/Characters/Player/Blueprints/BP_PlayerCharacter.Shields` _shields _playercharacter)
      (set `/Game/Characters/Player/Blueprints/BP_PlayerCharacter.Stamina` _stamina _playercharacter)
      (set `/Game/Characters/Player/Blueprints/Inventory/BP_Inventory.Weapons` _weapons _bp_inventory)
      (set `/Game/Characters/Player/Blueprints/Inventory/BP_Inventory.AmmoInventory` (`|MakeMap` "NewEnumerator0" _ammobullets "NewEnumerator4" _ammolasers "NewEnumerator5" _ammogrenade :!type "/Game/Characters/Player/Blueprints/Inventory/AmmoType Enum") _bp_inventory))
    (:`then_3`
      ;[1 1 1] Possess Char
      (`Controller.Possess` (`GameplayStatics.GetPlayerController` 0) (`self.PlayerCharacter`)))
    (:`then_4`
      (return _output_get))))

(fn `UserConstructionScript`)