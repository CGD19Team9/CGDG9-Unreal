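; LevelGoal is a level goal actor that shows an interaction UI while the player is within its box trigger.
; On overlap it passes itself to BP_PlayerCharacter, sets WithinRange and creates a new Wgt_LevelGoal on screen.
; On end overlap it clears WithinRange and hides that widget rather than removing it.
; Two DoOnce gates reset each other through ResetHide and ResetVisable, so show and hide alternate.
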(event `ResetVisable`
  ;[1 1 1] Show Interaction UI on Player Overlap
  (goto _label :!via `Reset`))

(event `self.Box.OnComponentBeginOverlap`
  (params (OverlappedComponent :type "PrimitiveComponent Object Reference") (OtherActor :type "Actor Object Reference") (OtherComp :type "PrimitiveComponent Object Reference") (OtherBodyIndex :type Integer) (bFromSweep :type Boolean) (SweepResult :type "HitResult Structure (by ref)"))
  ;[1 1 1] Show Interaction UI on Player Overlap
  (`/Engine/EditorBlueprintResources/StandardMacros.DoOnce` false :!label _label
    (:`Completed`
      (bind _asbp_player_character (cast `/Game/Characters/Player/Blueprints/BP_PlayerCharacter` OtherActor))
      (set `/Game/Characters/Player/Blueprints/BP_PlayerCharacter.Level Goal` self _asbp_player_character)
      (`/Engine/EditorBlueprintResources/StandardMacros.IsValid` _asbp_player_character
        (:`Is Valid`
          (set `self.withinRange?` true)
          (`self.ActivateGoal`)
          (`self.ResetHide`))))))

(event `self.Box.OnComponentEndOverlap`
  (params (OverlappedComponent :type "PrimitiveComponent Object Reference") (OtherActor :type "Actor Object Reference") (OtherComp :type "PrimitiveComponent Object Reference") (OtherBodyIndex :type Integer))
  ;[1 1 1] Hide Interaction UI on End Overlap
  (`/Engine/EditorBlueprintResources/StandardMacros.DoOnce` true :!label _label_2
    (:`Completed`
      (bind _asbp_player_character (cast `/Game/Characters/Player/Blueprints/BP_PlayerCharacter` OtherActor))
      (`/Engine/EditorBlueprintResources/StandardMacros.IsValid` _asbp_player_character
        (:`Is Valid`
          (set `self.withinRange?` false)
          (`self.DeactivateGoal`)
          (`self.ResetVisable`))))))

(event `ResetHide`
  ;[1 1 1] Hide Interaction UI on End Overlap
  (goto _label_2 :!via `Reset`))

(fn `ActivateGoal`
  ;[1 1 1] Add UI to Player Screen
  (bind _returnvalue (`|CreateWidget` "/Game/UI/Wgt_LevelGoal.Wgt_LevelGoal_C" (`GameplayStatics.GetPlayerController` 0)))
  (bind _output_get (set `self.Wgt_Reference` _returnvalue))
  (`UserWidget.AddToPlayerScreen` _output_get 0))

(fn `DeactivateGoal`
  ;[1 1 1] Hide UI
  (`Widget.SetVisibility` (`self.Wgt_Reference`) "Hidden"))

(fn `UserConstructionScript`)