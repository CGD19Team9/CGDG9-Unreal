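; BP_Pickup is a world pickup that offers a weapon, powerup or ammo to any actor overlapping its box.
; It sends type, ammo type, count and weapon class through a PickupItem message, destroying itself and its child actor if accepted.
; A DoOnce blocks repeat triggers and resets when the offer is not accepted.
; The construction script previews weapons as a child actor and shows a sphere for powerups and ammo.
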(event `self.Box.OnComponentBeginOverlap`
  (params (OverlappedComponent :type "PrimitiveComponent Object Reference") (OtherActor :type "Actor Object Reference") (OtherComp :type "PrimitiveComponent Object Reference") (OtherBodyIndex :type Integer) (bFromSweep :type Boolean) (SweepResult :type "HitResult Structure (by ref)"))
  (`/Engine/EditorBlueprintResources/StandardMacros.DoOnce` false :!label _label
    (:`Completed`
      (bind _success (message `/Game/Characters/Player/Blueprints/CharacterInterface.PickupItem` OtherActor (`self.PickupType`) (`self.AmmoType`) (`self.Count`) (`self.WeaponClass`)))
      (if _success
        (`ActorComponent.K2_DestroyComponent` (`self.ChildActor`))
        (`self.K2_DestroyActor`)
        (else
          (goto _label :!via `Reset`))))))

(fn `UserConstructionScript`
  (switch `/Game/Characters/Player/Blueprints/Inventory/PickupType` (`self.PickupType`)
    (:`NewEnumerator0`
      (`ChildActorComponent.SetChildActorClass` (`self.ChildActor`) (`self.WeaponClass`))
      (`SceneComponent.SetVisibility` (`self.ChildActor`) true true))
    (:`NewEnumerator1`
      (`SceneComponent.SetVisibility` (`self.Sphere`) true true :!label _label))
    (:`NewEnumerator2`
      (goto _label))))