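; LevelZones is a level zone actor that flags whether its area is safe from enemies.
; A looping five-second timer runs AreaScan, a sphere trace around the actor's location against target enemy object types with persistent debug drawing.
; The hit actor is cast to EnemyPawn_Parent before Safe is set.
; A failed cast ends the scan, so Safe stays unchanged when no enemy is hit.
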(event `self.ReceiveBeginPlay`
  (`KismetSystemLibrary.K2_SetTimer` null "AreaScan" 5.0 true))

(event `AreaScan`
  (bind _returnvalue (`self.K2_GetActorLocation` self))
  (bind _outhit (`KismetSystemLibrary.SphereTraceSingleForObjects` :`Start` _returnvalue :`End` _returnvalue :`Radius` (`self.ScanRadus`) :`ObjectTypes` (`self.TargetEnemies`) :`DrawDebugType` "Persistent"))
  (bind (_bblockinghit _binitialoverlap _time _distance _location _impactpoint _normal _impactnormal _physmat _hitactor) (`GameplayStatics.BreakHitResult` _outhit))
  (bind _asenemy_pawn_parent (cast `/Game/Characters/Enemies/Blueprints/EnemyPawn_Parent` _hitactor))
  (if (or (== _hitactor null) (!= _hitactor _asenemy_pawn_parent))
    (set `self.Safe?` true)
    (else
      (set `self.Safe?` false))))

(fn `UserConstructionScript`)