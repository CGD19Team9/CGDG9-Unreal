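; BP_Locker is a configurable locker prop that builds its look in the construction script, with no active event logic.
; BigLocker takes priority, then IsBroken picks one of two random broken meshes, otherwise IsOpen selects the open or closed mesh.
; SetColourScheme tints two dynamic paint materials from a palette map keyed by scheme and slot.
; It also sets a fixed polymer material and a green or red light material following IsOpen.
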(fn `UserConstructionScript`
  (bind _lockermesh (`self.LockerMesh`))
  (`|ExecutionSequence`
    (:`then_0`
      (if (`self.BigLocker?`)
        (`StaticMeshComponent.SetStaticMesh` (`self.LockerMesh`) "/Game/Props/SM_BigLocker.SM_BigLocker")
        (elif (`self.IsBroken?`)
          (`self.GetRandomMesh`)
          (elif (`self.IsOpen?`)
            (`StaticMeshComponent.SetStaticMesh` _lockermesh "/Game/Props/SM_OpenLocker.SM_OpenLocker")
            (else
              (`StaticMeshComponent.SetStaticMesh` _lockermesh "/Game/Props/SM_Locker.SM_Locker"))))))
    (:`then_1`
      (`self.SetColourScheme`))))