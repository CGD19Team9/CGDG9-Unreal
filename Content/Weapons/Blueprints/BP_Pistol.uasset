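; BP_Pistol is a hitscan pistol weapon Blueprint that damages the actor it hits.
; PrimaryFire line-traces for objects from an Arrow component along its forward vector out to Range, with timed debug drawing, then applies PrimaryDamage to the hit actor.
; SecondaryFire runs the same trace and damage path, so both fire modes behave identically.
; The construction script only calls its parent.
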(event `self.PrimaryFire`
  (bind _arrow (`self.Arrow`))
  (bind _returnvalue (`SceneComponent.K2_GetComponentLocation` _arrow))
  (bind _outhit (`KismetSystemLibrary.LineTraceSingleForObjects` :`Start` _returnvalue :`End` (+ _returnvalue (* (`SceneComponent.GetForwardVector` _arrow) (`self.Range`))) :`ObjectTypes` (`|MakeArray` "ObjectTypeQuery1" "ObjectTypeQuery2" "ObjectTypeQuery7" :!type "EObjectTypeQuery Enum") :`DrawDebugType` "ForDuration" :!label _label))
  (`GameplayStatics.ApplyDamage` (`.HitActor` (`GameplayStatics.BreakHitResult` _outhit)) (`self.PrimaryDamage`)))

(event `self.SecondaryFire`
  (goto _label))

(fn `UserConstructionScript`
  (`parent.UserConstructionScript`))