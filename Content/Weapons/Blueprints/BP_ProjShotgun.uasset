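; BP_ProjShotgun is a projectile shotgun weapon that fires a burst of BP_BaseProjectile pellets.
; PrimaryFire and SecondaryFire both set Spread from MaxSpreadPrimary and share one spawn loop, so they currently behave identically.
; Each pellet spawns at the Arrow component with random pitch and yaw within the spread.
; Pellet damage is computed as BulletsToFire divided by PrimaryDamage.
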(event `self.PrimaryFire`
  (bind _spread (`self.Spread`))
  (bind _returnvalue (* _spread -1.0))
  ;[1 1 1] Set Spread for Primary
  (set `self.Spread` (`self.MaxSpreadPrimary`))
  (for _ (range (+ (`KismetMathLibrary.FTrunc` (`self.BulletsToFire`)) 1)) :!label _label
    (`|SpawnActorFromClass` "/Game/Weapons/Blueprints/BP_BaseProjectile.BP_BaseProjectile_C" (`KismetMathLibrary.MakeTransform` (.location (`SceneComponent.K2_GetComponentToWorld` (`self.Arrow`))) (`KismetMathLibrary.MakeRotator` (.roll (.rotation (`SceneComponent.K2_GetComponentToWorld` (`self.Arrow`)))) (+ (.pitch (.rotation (`SceneComponent.K2_GetComponentToWorld` (`self.Arrow`)))) (`KismetMathLibrary.RandomFloatInRange` _returnvalue _spread)) (+ (.yaw (.rotation (`SceneComponent.K2_GetComponentToWorld` (`self.Arrow`)))) (`KismetMathLibrary.RandomFloatInRange` _returnvalue _spread))) (.scale (`SceneComponent.K2_GetComponentToWorld` (`self.Arrow`)))) "Undefined" "OverrideRootScale" self (/ (`self.BulletsToFire`) (`self.PrimaryDamage`)) null)))

(event `self.SecondaryFire`
  ;[1 1 1] Set Spread for Secondary
  (set `self.Spread` (`self.MaxSpreadPrimary`))
  (goto _label))

(fn `UserConstructionScript`
  (`parent.UserConstructionScript`))