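; Base weapon Blueprint that fires projectiles and manages clip and reserve ammo through an inventory reference.
; FireWeapon refreshes ammo from the inventory, spends clip rounds and spawns a primary projectile, or a secondary one when aiming, at the Arrow transform with damage passed in.
; A DoOnce with delayed reset throttles secondary fire.
; An insufficient clip triggers a timed Reload, which deducts inventory ammo and writes the clip count back.
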(event `Reload`
  (bind _maxclipsize (`self.MaxClipSize`))
  (bind _inventoryref (`self.InventoryRef`))
  ;[1 1 1] Reload
  (if (and (!= (`self.Ammo`) 0) (not (`self.Reloading`)))
    (set `self.Reloading` true)
    (`KismetSystemLibrary.PrintString` "RELOADING" true false (struct :`R` 1.0 :`G` 0.134413 :`B` 0.706118 :`A` 1.0))
    (`KismetSystemLibrary.Delay` (`self.ReloadTime`))
    (`|ExecutionSequence`
      (:`then_0`
        (if (> (- (`self.MaxClipSize`) (`self.Clip`)) (`self.Ammo`))
          ;;[1 1 1] Not enough for max clip
          (bind _output_get (set `self.Clip` (`self.Ammo`)))
          (`/Game/Characters/Player/Blueprints/Inventory/BP_Inventory.RemoveAmmo` _inventoryref (`self.AmmoType`) _output_get)
          (set `self.Ammo` 0)
          (else
            ;;[1 1 1] Enough Ammo
            (set `self.Clip` (`self.MaxClipSize`))
            (`/Game/Characters/Player/Blueprints/Inventory/BP_Inventory.RemoveAmmo` _inventoryref (`self.AmmoType`) _maxclipsize)
            (set `self.Ammo` (- (`self.Ammo`) _maxclipsize))))
        (`/Game/Characters/Player/Blueprints/Inventory/BP_Inventory.SetClip` (`self.InventoryRef`) (`GameplayStatics.GetObjectClass` self) (`self.Clip`)))
      (:`then_1`
        (set `self.Reloading` false)))))

(event `/Game/Weapons/Blueprints/WeaponInterface.SetClip`
  (params (Clip :type Integer) (SetMaxClip :type Boolean))
  (bind _output_get (set `self.Clip` (select `bool` SetMaxClip :`false` Clip :`true` (`self.MaxClipSize`))))
  (if (< _output_get 0)
    (set `self.Clip` 0)))

(event `/Game/Weapons/Blueprints/WeaponInterface.FireWeapon`
  (params (Inventory :type "/Game/Characters/Player/Blueprints/Inventory/BP_Inventory Object Reference"))
  (bind _returnvalue (- (`self.Clip`) (`self.PrimaryAmmoCost`)))
  (bind _returnvalue_2 (- (`self.Clip`) (`self.SecondaryAmmoCost`)))
  (if (not (`self.Reloading`))
    (bind _output_get (set `self.InventoryRef` Inventory))
    (`/Game/Characters/Player/Blueprints/Inventory/BP_Inventory.GetAmmo` Inventory (`self.AmmoType`))
    (bind _count (`/Game/Characters/Player/Blueprints/Inventory/BP_Inventory.GetAmmo` _output_get (`self.AmmoType`)))
    (set `self.Ammo` _count)
    (`KismetSystemLibrary.PrintString` (`KismetStringLibrary.Concat_StrStr` "Ammo: " (`KismetStringLibrary.Conv_IntToString` (`self.Ammo`)) "Clip: " (`KismetStringLibrary.Conv_IntToString` (`self.Clip`))) true true (struct :`R` 1.0 :`G` 0.203959 :`B` 0.829131 :`A` 1.0))
    (`|ExecutionSequence`
      (:`then_0`
        (if (> (`self.Clip`) 0)
          (if (`self.isAiming`)
            (`/Engine/EditorBlueprintResources/StandardMacros.DoOnce` false :!label _label
              (:`Completed`
                (if (< _returnvalue_2 0)
                  (`self.Reload`)
                  (else
                    (set `self.Clip` _returnvalue_2)
                    (bind _returnvalue_3 (`|SpawnActorFromClass` (`self.SecondaryProjectile`) (`SceneComponent.K2_GetComponentToWorld` (`self.Arrow`)) "AlwaysSpawn" "OverrideRootScale" self null))
                    (message `/Game/Weapons/Blueprints/WeaponInterface.SetDamage` _returnvalue_3 (`self.SecondaryDamage`))
                    (`KismetSystemLibrary.Delay` 1.5)
                    (goto _label :!via `Reset`)))))
            (elif (< _returnvalue 0)
              (`self.Reload`)
              (else
                (set `self.Clip` _returnvalue)
                (bind _returnvalue_4 (`|SpawnActorFromClass` (`self.PrimaryProjectile`) (`SceneComponent.K2_GetComponentToWorld` (`self.Arrow`)) "AlwaysSpawn" "OverrideRootScale" null null))
                (message `/Game/Weapons/Blueprints/WeaponInterface.SetDamage` _returnvalue_4 (`self.PrimaryDamage`)))))
          (else
            (`self.Reload`))))
      (:`then_1`
        (`/Game/Characters/Player/Blueprints/Inventory/BP_Inventory.SetClip` (`self.InventoryRef`) (`GameplayStatics.GetObjectClass` self) (`self.Clip`))))))

(event `/Game/Weapons/Blueprints/WeaponInterface.Aiming`
  (params (`Aiming?` :type Boolean))
  (set `self.isAiming` `Aiming?`))

(fn `UserConstructionScript`)