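; Base hammer weapon Blueprint that damages actors overlapping its Box component after a one-second delay.
; A custom event toggles a FlipFlop whose state gates the overlap response; its A output also runs the hit logic directly.
; While aiming, a hit deals heavier damage and slightly offsets the target's local transform using Arrow0's forward vector; otherwise it only applies lighter damage.
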(event `CustomEvent`
  (bind _isa (`/Engine/EditorBlueprintResources/StandardMacros.FlipFlop`)
    (:`A`
      (if (`self.isAiming`) :!label _label
        (`KismetSystemLibrary.Delay` 1.0)
        (`GameplayStatics.ApplyDamage` (stale `self.Box.OnComponentBeginOverlap` OtherActor) 30.0)
        (`self.K2_AddActorLocalTransform` (stale `self.Box.OnComponentBeginOverlap` OtherActor) (`KismetMathLibrary.Conv_VectorToTransform` (* (`SceneComponent.GetForwardVector` (`self.Arrow_0`)) (0.1 0.1 0.1))) false false)
        (else
          (`KismetSystemLibrary.Delay` 1.0)
          (`GameplayStatics.ApplyDamage` (stale `self.Box.OnComponentBeginOverlap` OtherActor) 10.0))))))

(event `self.Box.OnComponentBeginOverlap`
  (params (OverlappedComponent :type "PrimitiveComponent Object Reference") (OtherActor :type "Actor Object Reference") (OtherComp :type "PrimitiveComponent Object Reference") (OtherBodyIndex :type Integer) (bFromSweep :type Boolean) (SweepResult :type "HitResult Structure (by ref)"))
  (if (stale `CustomEvent` _isa)
    (goto _label)))

(fn `UserConstructionScript`)