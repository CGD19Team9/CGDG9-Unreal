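; BP_ProjPistol is a projectile pistol weapon Blueprint with primary and secondary fire modes.
; Primary fire spawns a BP_BaseProjectile at the Arrow component's transform, then spawns a second after a short delay for a two-shot burst.
; Secondary fire spawns a single BP_BaseProjectileAim from the same Arrow transform.
; Each mode passes its own damage value to the projectile, and spawns ignore collisions.
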(event `self.PrimaryFire`
  ;[1 1 1] Primary Fire - Shoots twice
  (`|ExecutionSequence`
    (:`then_0`
      _)
    (:`then_1`
      (`KismetSystemLibrary.Delay` 0.1)))
  (`|SpawnActorFromClass` "/Game/Weapons/Blueprints/BP_BaseProjectile.BP_BaseProjectile_C" (`SceneComponent.K2_GetComponentToWorld` (`self.Arrow`)) "AlwaysSpawn" "OverrideRootScale" null (`self.PrimaryDamage`) null))

(event `self.SecondaryFire`
  ;[1 1 1] Secondary Fire
  (`|SpawnActorFromClass` "/Game/Weapons/Blueprints/BP_BaseProjectileAim.BP_BaseProjectileAim_C" (`SceneComponent.K2_GetComponentToWorld` (`self.Arrow`)) "AlwaysSpawn" "OverrideRootScale" null (`self.SecondaryDamage`) null))

(fn `UserConstructionScript`
  (`parent.UserConstructionScript`))