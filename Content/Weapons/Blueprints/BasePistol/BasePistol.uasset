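; Base pistol weapon with a custom fire event that spawns projectiles from its Arrow's transform and spends Clip rounds.
; Aimed shots spawn a separate aim projectile, throttled by a DoOnce that resets after a delay, while unaimed shots have no cooldown.
; An empty clip triggers a delayed reload of a full magazine from Ammo, then loops back to fire.
; All firing requires Ammo above zero, even with rounds in the clip.
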(event `CustomEvent`
  (if (> (`self.Ammo`) 0) :!label _label
    (if (> (`self.Clip`) 0)
      (if (`self.isAiming`)
        (`KismetSystemLibrary.PrintString` "Slowshot")
        (`/Engine/EditorBlueprintResources/StandardMacros.DoOnce` false :!label _label_2
          (:`Completed`
            (`|SpawnActorFromClass` "/Game/Weapons/Blueprints/BP_BaseProjectileAim.BP_BaseProjectileAim_C" (`SceneComponent.K2_GetComponentToWorld` (`self.Arrow`)) "AlwaysSpawn" "OverrideRootScale" null 12.0 null)
            (bind _result (`/Engine/EditorBlueprintResources/StandardMacros.DecrementInt` (`self.Clip`))
              (:`  `
                (set `self.Clip` _result)
                (`KismetSystemLibrary.Delay` 1.5)
                (goto _label_2 :!via `Reset`)))))
        (else
          (`|SpawnActorFromClass` "/Game/Weapons/Blueprints/BP_BaseProjectile.BP_BaseProjectile_C" (`SceneComponent.K2_GetComponentToWorld` (`self.Arrow`)) "AlwaysSpawn" "OverrideRootScale" null null)
          (bind _result_2 (`/Engine/EditorBlueprintResources/StandardMacros.DecrementInt` (`self.Clip`))
            (:`  `
              (set `self.Clip` _result_2)))))
      (else
        (`KismetSystemLibrary.PrintString` "Reload")
        (`KismetSystemLibrary.Delay` 1.5)
        (set `self.Ammo` (- (`self.Ammo`) (`self.MaxClipSize`)))
        (set `self.Clip` (+ (`self.Clip`) (`self.MaxClipSize`)))
        (goto _label)))))

(fn `UserConstructionScript`)