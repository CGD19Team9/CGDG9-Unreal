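; ExpLauncher is an explosive launcher weapon Blueprint that fires projectiles only while aiming.
; A custom event checks ammo, clip and aim state, then spawns an ExpLauncherProjectileAim at the Arrow's transform and decrements the clip.
; A DoOnce reset after a delay limits fire rate.
; An empty clip triggers a delayed reload from reserve ammo that loops back into the firing checks, with debug prints for blocked states.
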(event `CustomEvent`
  (if (> (`self.Ammo`) 0) :!label _label
    (if (> (`self.Clip size`) 0)
      (if (`self.isAiming`)
        (`/Engine/EditorBlueprintResources/StandardMacros.DoOnce` false :!label _label_2
          (:`Completed`
            (`|SpawnActorFromClass` "/Game/Weapons/Blueprints/BaseExplosiveLauncher/ExpLauncherProjectileAim.ExpLauncherProjectileAim_C" (`SceneComponent.K2_GetComponentToWorld` (`self.Arrow`)) "Undefined" "OverrideRootScale" null null)
            (bind _result (`/Engine/EditorBlueprintResources/StandardMacros.DecrementInt` (`self.Clip size`))
              (:`  `
                (set `self.Clip size` _result)
                (`KismetSystemLibrary.Delay` 1.0)
                (goto _label_2 :!via `Reset`)))))
        (else
          (`KismetSystemLibrary.PrintString` "Only Fire While Aiming")))
      (else
        (`KismetSystemLibrary.PrintString` "Reload")
        (`KismetSystemLibrary.Delay` 1.5)
        (set `self.Ammo` (- (`self.Ammo`) (`self.MaxClipSize`)))
        (set `self.Clip size` (+ (`self.Clip size`) (`self.MaxClipSize`)))
        (goto _label)))
    (else
      (`KismetSystemLibrary.PrintString` "Out of Ammo"))))

(fn `UserConstructionScript`)