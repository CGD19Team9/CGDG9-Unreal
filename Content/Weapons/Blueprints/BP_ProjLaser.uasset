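; Laser weapon Blueprint with primary and secondary fire modes that shoot separate projectile actors.
; Primary fire spawns BP_Laser1 and secondary fire spawns BP_Laser2 at the Arrow component's world transform, ignoring spawn collisions.
; Each spawned laser receives the damage value of its fire mode as its base damage.
; The construction script only calls the parent's.
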(event `self.PrimaryFire`
  (`|SpawnActorFromClass` "/Game/Weapons/Blueprints/Projectiles/BP_Laser1.BP_Laser1_C" (`SceneComponent.K2_GetComponentToWorld` (`self.Arrow`)) "AlwaysSpawn" "OverrideRootScale" null (`self.PrimaryDamage`) null))

(event `self.SecondaryFire`
  (`|SpawnActorFromClass` "/Game/Weapons/Blueprints/Projectiles/BP_Laser2.BP_Laser2_C" (`SceneComponent.K2_GetComponentToWorld` (`self.Arrow`)) "AlwaysSpawn" "OverrideRootScale" null (`self.SecondaryDamage`) null))

(fn `UserConstructionScript`
  (`parent.UserConstructionScript`))