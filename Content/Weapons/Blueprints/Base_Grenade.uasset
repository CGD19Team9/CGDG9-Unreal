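; Base grenade actor that deals radial falloff damage when it explodes, then destroys itself.
; A timer started at BeginPlay triggers the explosion, as does a Sphere hit when ExplodeOnImpact is set.
; DoOnce guards against repeat detonation, and an empty OnExplode event receives the blast location as a hook before destruction.
; A debug "POP" string prints on detonation.
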(event `OnExplode`
  (params (ExplodeLocation :type "Vector Structure")))

(event `Explode`
  (bind _returnvalue (`SceneComponent.K2_GetComponentLocation` (`self.Sphere`)))
  (`/Engine/EditorBlueprintResources/StandardMacros.DoOnce` false
    (:`Completed`
      (`GameplayStatics.ApplyRadialDamageWithFalloff` (`self.BaseDamage`) (`self.MinimumDamage `) _returnvalue (`self.Damage Inner Radius`) (`self.Damage Outer Radius`) (`self.Damage Falloff `) null (`|MakeArray` self :!type "Actor Object Reference") null null)
      (`KismetSystemLibrary.PrintString` "POP" true false)
      (`self.OnExplode` _returnvalue)
      (`self.K2_DestroyActor`))))

(event `self.ReceiveBeginPlay`
  (`KismetSystemLibrary.Delay` (`self.TimeTilExplode`))
  (`self.Explode`))

(event `self.Sphere.OnComponentHit`
  (params (HitComponent :type "PrimitiveComponent Object Reference") (OtherActor :type "Actor Object Reference") (OtherComp :type "PrimitiveComponent Object Reference") (NormalImpulse :type "Vector Structure") (Hit :type "HitResult Structure (by ref)"))
  (if (`self.ExplodeOnImpact`)
    (`self.Explode`)))

(fn `UserConstructionScript`)