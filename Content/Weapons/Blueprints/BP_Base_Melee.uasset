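; Base Blueprint for melee weapons that spend player stamina to swing and damage actors the weapon overlaps.
; FireWeapon is gated by a DoOnce, deducts EnergyCost from the player character, opens an Attacking window for SwingSpeed while calling the empty PrimaryFire event, then re-arms after CoolDown.
; Capsule overlaps during that window apply damage once per actor via a Hit list, ending the window early unless multiple targets are allowed.
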(event `/Game/Weapons/Blueprints/WeaponInterface.FireWeapon`
  (params (Inventory :type "/Game/Characters/Player/Blueprints/Inventory/BP_Inventory Object Reference"))
  (`/Engine/EditorBlueprintResources/StandardMacros.DoOnce` false :!label _label
    (:`Completed`
      ;[1 1 1] If no energy reset
      (bind _success (`self.RemoveStamina`))
      (if _success
        (`|ExecutionSequence`
          (:`then_0`
            (`KismetArrayLibrary.Array_Clear` (`self.Hit`))
            (set `self.Attacking` true)
            (`self.PrimaryFire`)
            (`KismetSystemLibrary.Delay` (`self.SwingSpeed`))
            (set `self.Attacking` false)
            (`KismetArrayLibrary.Array_Clear` (`self.Hit`)))
          (:`then_1`
            ;[1 1 1] Reset after cooldown
            (`KismetSystemLibrary.Delay` (`self.CoolDown`))
            (`self.Fire Weapon Reset`)))
        (else
          (`self.Fire Weapon Reset`))))))

(event `Fire Weapon Reset`
  (goto _label :!via `Reset`))

(event `PrimaryFire`)

(event `self.CapsuleCollision.OnComponentBeginOverlap`
  (params (OverlappedComponent :type "PrimitiveComponent Object Reference") (OtherActor :type "Actor Object Reference") (OtherComp :type "PrimitiveComponent Object Reference") (OtherBodyIndex :type Integer) (bFromSweep :type Boolean) (SweepResult :type "HitResult Structure (by ref)"))
  ;[1 1 1] On Overlap
  (if (`self.Attacking`)
    (if (<= (`KismetArrayLibrary.Array_Find` (`self.Hit`) OtherActor) -1)
      (`GameplayStatics.ApplyDamage` OtherActor (`self.Damage`))
      (`KismetArrayLibrary.Array_AddUnique` (`self.Hit`) OtherActor)
      ;;[1 0 0.4817] Stops hitting mulitple
      (if (not (`self.CanHitMultipleTargets`))
        (set `self.Attacking` false)))))

(fn `GetAmmoType`
  (returns (AmmoType :type "/Game/Characters/Player/Blueprints/Inventory/AmmoType Enum"))
  (return "NewEnumerator0"))

(fn `RemoveStamina`
  (returns (Success :type Boolean))
  (bind _asbp_player_character (cast `/Game/Characters/Player/Blueprints/BP_PlayerCharacter` (`GameplayStatics.GetPlayerCharacter` 0))
    (:`then`
      (bind _stamina (`/Game/Characters/Player/Blueprints/BP_PlayerCharacter.Stamina` _asbp_player_character))
      (if (>= _stamina (`self.EnergyCost`))
        (set `/Game/Characters/Player/Blueprints/BP_PlayerCharacter.Stamina` (- _stamina (`self.EnergyCost`)) _asbp_player_character)
        (return true)
        (else
          (return false))))
    (:`CastFailed`
      (return false))))

(fn `UserConstructionScript`)