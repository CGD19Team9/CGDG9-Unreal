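; BP_Shotgun is a shotgun weapon whose primary and secondary fire events run the same hitscan pellet logic.
; Each shot fires BulletsToFire object traces from the Arrow component out to Range, randomly offsetting each endpoint per world axis within MaxSpread.
; Each trace applies an equal share of PrimaryDamage to its hit actor and draws a timed debug line.
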(event `self.PrimaryFire`
  (bind _arrow (`self.Arrow`))
  (bind _maxspread (`self.MaxSpread`))
  (bind _returnvalue (`SceneComponent.K2_GetComponentLocation` _arrow))
  (bind _returnvalue_2 (* _maxspread -1.0))
  (for _ (range (+ (`KismetMathLibrary.FTrunc` (`self.BulletsToFire`)) 1)) :!label _label
    (bind _outhit (`KismetSystemLibrary.LineTraceSingleForObjects` :`Start` _returnvalue :`End` (`KismetMathLibrary.MakeVector` (+ (.x (+ _returnvalue (* (`SceneComponent.GetForwardVector` _arrow) (`self.Range`)))) (`KismetMathLibrary.RandomFloatInRange` _returnvalue_2 _maxspread)) (+ (.y (+ _returnvalue (* (`SceneComponent.GetForwardVector` _arrow) (`self.Range`)))) (`KismetMathLibrary.RandomFloatInRange` _returnvalue_2 _maxspread)) (+ (.z (+ _returnvalue (* (`SceneComponent.GetForwardVector` _arrow) (`self.Range`)))) (`KismetMathLibrary.RandomFloatInRange` _returnvalue_2 _maxspread))) :`ObjectTypes` (`|MakeArray` "ObjectTypeQuery1" "ObjectTypeQuery2" "ObjectTypeQuery7" :!type "EObjectTypeQuery Enum") :`DrawDebugType` "ForDuration" :`TraceHitColor` (struct :`G` 1.0) :`DrawTime` 1.0))
    (`GameplayStatics.ApplyDamage` (`.HitActor` (`GameplayStatics.BreakHitResult` _outhit)) (/ (`self.PrimaryDamage`) (`self.BulletsToFire`)))))

(event `self.SecondaryFire`
  (goto _label))

(fn `UserConstructionScript`
  (`parent.UserConstructionScript`))