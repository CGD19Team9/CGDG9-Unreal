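; Long laser weapon Blueprint that fires projectiles from an arrow component while ammo remains.
; Aimed fire spawns an aim projectile at a higher clip cost behind a DoOnce cooldown, while hip fire spawns standard projectiles in DoN-limited bursts with a shorter reset delay.
; An empty clip triggers a delayed reload from reserve ammo, then loops back to fire.
; The aimed shot's line trace result is unused.
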(event `/Game/Weapons/WeaponInterface.FireWeapon`
  (bind _returnvalue (`SceneComponent.GetForwardVector` (`self.LaserBarrel`)))
  (bind _returnvalue_2 (`SceneComponent.K2_GetComponentToWorld` (`self.Arrow`)))
  (if (> (`self.Ammo`) 0) :!label _label
    (if (> (`self.Clip size`) 0)
      (if (`self.isAiming`)
        (`/Engine/EditorBlueprintResources/StandardMacros.DoOnce` false :!label _label_2
          (:`Completed`
            (bind _outhit (`KismetSystemLibrary.LineTraceSingle` _returnvalue (+ _returnvalue 1000.0) "TraceTypeQuery1"))
            (`|SpawnActorFromClass` "/Game/Weapons/BaseLongLaser/BP_ProjectileLaserAim.BP_ProjectileLaserAim_C" _returnvalue_2 "AlwaysSpawn" "OverrideRootScale" null null)
            (set `self.Clip size` (- (`self.Clip size`) 3))
            (`KismetSystemLibrary.Delay` 3.0)
            (goto _label_2 :!via `Reset`)))
        (else
          (`/Engine/EditorBlueprintResources/StandardMacros.Do N` 3 :!label _label_3
            (:`Exit`
              (`|SpawnActorFromClass` "/Game/Weapons/BaseLongLaser/BP_LaserProjectile.BP_LaserProjectile_C" _returnvalue_2 "AlwaysSpawn" "OverrideRootScale" null null)
              (bind _result (`/Engine/EditorBlueprintResources/StandardMacros.DecrementInt` (`self.Clip size`))
                (:`  `
                  (set `self.Clip size` _result)
                  (`KismetSystemLibrary.Delay` 1.0)
                  (goto _label_3 :!via `Reset`)))))))
      (else
        (`KismetSystemLibrary.PrintString` "Reload")
        (`KismetSystemLibrary.Delay` 1.5)
        (set `self.Ammo` (- (`self.Ammo`) (`self.MaxClipSize`)))
        (set `self.Clip size` (+ (`self.Clip size`) (`self.MaxClipSize`)))
        (goto _label)))))

(fn `UserConstructionScript`
  (`parent.UserConstructionScript`))