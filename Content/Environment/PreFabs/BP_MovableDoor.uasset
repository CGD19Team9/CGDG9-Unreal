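; A movable door prefab that slides its static mesh vertically between closed and open positions.
; BeginPlay stores the mesh's relative location as closed, offsets Z by DoorMovementAmount for open, then immediately plays DoorMovementTimeline.
; The timeline's Alpha lerps the mesh's relative location between the two positions, without sweep.
; OpenDoor plays the timeline and CloseDoor reverses it; the construction script holds only disconnected position logic.
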(event `self.ReceiveBeginPlay`
  (`|ExecutionSequence`
    (:`then_0`
      (bind _output_get (set `self.ClosePosition` (`SceneComponent.RelativeLocation` (`self.StaticMesh`))))
      (set `self.OpenPosition` (`KismetMathLibrary.MakeVector` (.x _output_get) (.y _output_get) (+ (.z _output_get) (`self.DoorMovementAmount`)))))
    (:`then_1`
      (bind (_direction _alpha) (`Timeline|DoorMovementTimeline` :!label _label)
        (:`Update`
          (`SceneComponent.K2_SetRelativeLocation` (`self.StaticMesh`) (`KismetMathLibrary.VLerp` (`self.OpenPosition`) (`self.ClosePosition`) _alpha) false false))))))

(event `OpenDoor`
  (goto _label))

(event `CloseDoor`
  (goto _label :!via `Reverse`))

(fn `UserConstructionScript`)