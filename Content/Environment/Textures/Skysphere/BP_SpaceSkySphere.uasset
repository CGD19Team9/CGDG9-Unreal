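; BP_SpaceSkySphere is a placeable sky actor that, judging by its name, provides a space backdrop around the level.
; Its construction script uniformly scales SkyMesh by SkysphereScale and assigns six material variables to the mesh's slots, one each for back, top, right, left, bottom and front, cubemap-style.
; All setup happens at construction, and the event graph holds only disabled placeholder events.
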(fn `UserConstructionScript`
  (bind _skymesh (`self.SkyMesh`))
  (bind _skysphere_scale (`self.Skysphere Scale`))
  (`SceneComponent.SetWorldScale3D` (`self.SkyMesh`) (`KismetMathLibrary.MakeVector` _skysphere_scale _skysphere_scale _skysphere_scale))
  (`PrimitiveComponent.SetMaterial` _skymesh 0 (`self.SkySphereBack`))
  (`PrimitiveComponent.SetMaterial` _skymesh 1 (`self.SkySphereTop`))
  (`PrimitiveComponent.SetMaterial` _skymesh 2 (`self.SkySphereRight`))
  (`PrimitiveComponent.SetMaterial` _skymesh 3 (`self.SkySphereLeft`))
  (`PrimitiveComponent.SetMaterial` _skymesh 4 (`self.SkySphereBottom`))
  (`PrimitiveComponent.SetMaterial` _skymesh 5 (`self.SkySphereFront`)))