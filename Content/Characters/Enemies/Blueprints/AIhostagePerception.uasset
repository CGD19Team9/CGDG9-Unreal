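; Behavior tree service for hostage AI perception that switches the blackboard between targeting and path following.
; Each AI tick reads CanseePlayer from the owning AIControllerParent: when true, it clears MovementPath and writes AITarget to TargetPawn.
; Otherwise it writes the controller's CurrentPathNode to MovementPath, leaving TargetPawn untouched.
; Separate SetTarget and SetTargetLocation functions store a player and location in variables that the tick does not read.
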(event `self.ReceiveTickAI`
  (params (OwnerController :type "AIController Object Reference") (ControlledPawn :type "Pawn Object Reference") (DeltaSeconds :type "Float (single-precision)"))
  (bind _asaicontroller_parent (cast `/Game/Characters/Enemies/Blueprints/AIControllerParent` OwnerController))
  (if (`/Game/Characters/Enemies/Blueprints/AIControllerParent.canseePlayer?` _asaicontroller_parent)
    (`BTFunctionLibrary.ClearBlackboardValue` (`self.MovementPath`))
    (`BTFunctionLibrary.SetBlackboardValueAsObject` (`self.TargetPawn`) (`/Game/Characters/Enemies/Blueprints/AIControllerParent.AITarget` _asaicontroller_parent))
    (else
      (`BTFunctionLibrary.SetBlackboardValueAsObject` (`self.MovementPath`) (`/Game/Characters/Enemies/Blueprints/AIControllerParent.CurrentPathNode` _asaicontroller_parent)))))

(fn `SetTarget`
  (params (Player :type "/Game/Characters/Player/Blueprints/BP_PlayerCharacter Object Reference"))
  (set `self.TargetPlayer` Player))

(fn `SetTargetLocation`
  (params (TargetLoc :type "Vector Structure"))
  (set `self.TargetLocation` TargetLoc))