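; EnemyPawnBP is an enemy pawn that deals melee damage to the player character.
; An overlap on its PHWeapon component casts the other actor to BP_PlayerCharacter and calls Attack, which applies MeleeDamage.
; A DoOnce gate, reset after an AttackRate delay, limits hit frequency; attacks trigger only on overlap begin, and CanAttack is set but never read here.
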(event `self.PHWeapon.OnComponentBeginOverlap`
  (params (OverlappedComponent :type "PrimitiveComponent Object Reference") (OtherActor :type "Actor Object Reference") (OtherComp :type "PrimitiveComponent Object Reference") (OtherBodyIndex :type Integer) (bFromSweep :type Boolean) (SweepResult :type "HitResult Structure (by ref)"))
  ;[1 1 1] Check if Overlapped and canAttack, then reset attack function using attck rate
  (bind _asbp_player_character (cast `/Game/Characters/Player/Blueprints/BP_PlayerCharacter` OtherActor))
  (set `self.canAttack?` true)
  (`/Engine/EditorBlueprintResources/StandardMacros.DoOnce` false :!label _label
    (:`Completed`
      (`self.Attack` _asbp_player_character)
      (`KismetSystemLibrary.Delay` (`self.AttackRate`))
      (`self.ResetAttack`))))

(event `ResetAttack`
  ;[1 1 1] Check if Overlapped and canAttack, then reset attack function using attck rate
  (goto _label :!via `Reset`))

(fn `Attack`
  (params (TargettedActor :type "/Game/Characters/Player/Blueprints/BP_PlayerCharacter Object Reference"))
  ;[1 1 1] Apply Damage to Target
  (`GameplayStatics.ApplyDamage` TargettedActor (`self.MeleeDamage`) null self))

(fn `UserConstructionScript`)