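; Little Muscle enemy pawn, a child enemy Blueprint that deals melee damage to the player.
; BeginPlay runs the parent logic, then copies its Set variables into the working particle, health, attack rate, run speed and armour values and assigns its enemy type.
; The Attack event finds player characters overlapping PHWeapon and applies melee damage after an AttackRate delay, placed inside the loop.
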(event `self.ReceiveBeginPlay`
  (`parent.ReceiveBeginPlay`)
  (set `self.UpdatedParticle` (`self.SetParticle`))
  (set `self.TotalHP` (`self.Set HP`))
  (set `self.AttackRate` (`self.Set Attack Rate`))
  (set `self.RunSpeed` (`self.Set Run Speed`))
  (set `self.Armour` (`self.Set Armour`))
  (set `self.Type` "NewEnumerator1"))

(event `/Game/Characters/Enemies/Blueprints/Int_AIFunc.Attack`
  (for _array_element (`PrimitiveComponent.GetOverlappingActors` (`self.PHWeapon`) "/Game/Characters/Player/Blueprints/BP_PlayerCharacter.BP_PlayerCharacter_C")
    (`KismetSystemLibrary.Delay` (`self.AttackRate`))
    (`GameplayStatics.ApplyDamage` _array_element (`self.MeleeDamage`))))

(fn `UserConstructionScript`
  (`parent.UserConstructionScript`))