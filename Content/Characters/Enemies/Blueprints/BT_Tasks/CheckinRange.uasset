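; Behavior tree task that checks whether the controlled EP_Parent enemy has an EP_Hostage within its WeaponRange.
; On execute, it gathers all hostages and compares the enemy's distance to each against that range.
; A hit sets Range and the InRange blackboard key to true and finishes successfully, while a miss finishes as failed without clearing the key.
; FinishExecute runs inside the unbroken loop, so it never fires when no hostages exist.
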(event `self.ReceiveExecuteAI`
  (params (OwnerController :type "AIController Object Reference") (ControlledPawn :type "Pawn Object Reference"))
  (bind _asep_parent (cast `/Game/Characters/Enemies/Blueprints/Classes/EP_Parent` ControlledPawn))
  (bind _outactors (`GameplayStatics.GetAllActorsOfClass` "/Game/Characters/Enemies/Blueprints/Classes/EP_Hostage.EP_Hostage_C"))
  (for _array_element _outactors
    (if (<= (`Actor.GetDistanceTo` _asep_parent _array_element) (`/Game/Characters/Enemies/Blueprints/Classes/EP_Parent.WeaponRange` _asep_parent))
      (set `self.Range` true)
      (`BTFunctionLibrary.SetBlackboardValueAsBool` (`self.inRange`) true)
      (`self.FinishExecute` true)
      (else
        (`self.FinishExecute` false)))))