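; Behavior Tree task that moves an enemy to a blackboard location, using the pawn's weapon range as the acceptance radius.
; If the AI controller can see the player, it waits briefly and fails instead of moving.
; Otherwise it runs AIMoveTo, whose immediate exec pin and Success both finish the task as successful, so it does not wait for arrival; Fail reports failure.
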(event `self.ReceiveExecuteAI`
  (params (OwnerController :type "AIController Object Reference") (ControlledPawn :type "Pawn Object Reference"))
  ;[1 1 1] Get Loc Entry and Move to Target, account for weapon range (if applicable)
  (bind _asaicontroller_parent (cast `/Game/Characters/Enemies/Blueprints/Misc/AIControllerParent` OwnerController))
  (bind _asep_parent (cast `/Game/Characters/Enemies/Blueprints/Classes/EP_Parent` (`Controller.K2_GetPawn` _asaicontroller_parent)))
  (if (`/Game/Characters/Enemies/Blueprints/Misc/AIControllerParent.canseePlayer?` _asaicontroller_parent)
    (`KismetSystemLibrary.Delay` 1.0)
    (`self.FinishExecute` false)
    (else
      (`|AIMoveTo` ControlledPawn (`BlackboardComponent.GetLocationFromEntry` (`BTFunctionLibrary.GetOwnersBlackboard`) (`self.MoveKey`)) null (`/Game/Characters/Enemies/Blueprints/Classes/EP_Parent.WeaponRange` _asep_parent)
        (:`then`
          (`self.FinishExecute` true :!label _label))
        (:`OnSuccess`
          (goto _label))
        (:`OnFail`
          (`self.FinishExecute` false))))))