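; Parent AI controller for enemy and hostage pawns that possesses its pawn, starts the hostage behavior tree and handles awareness and pathing.
; Looping timers capsule-trace for players, hostages or enemies, pick a random spawn-point path node, and update safe zones for hostages.
; Obstacle line traces confirm sight, set targets and message the pawn to chase or follow its path.
; Type-based behavior tree selection exists but is disconnected.
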(event `self.ReceiveBeginPlay`
  (bind _returnvalue (`self.K2_GetPawn`))
  ;[1 1 1] Possess Pawns on Spawn and Run AI Awareness
  (`self.PossessAIPawns`)
  (bind _outactors (`GameplayStatics.GetAllActorsOfClass` "/Game/Base/Blueprints/enemySpawnPoint.EnemySpawnPoint_C"))
  (for _array_element _outactors
    (`KismetArrayLibrary.Array_Add` (`self.EnemySpawnstoIgnore`) _array_element))
  (`self.RunBehaviorTree` "/Game/Characters/Enemies/Blueprints/HostageAI_BT.HostageAI_BT")
  (bind _returnvalue_2 (`KismetSystemLibrary.K2_SetTimer` null "CheckforPlayer" 0.5 true))
  (set `self.AIPerceptionHandle` _returnvalue_2)
  (bind _returnvalue_3 (`KismetSystemLibrary.K2_SetTimer` null "GetNewPath" 2.0 true))
  (set `self.PathingTimerHandle` _returnvalue_3)
  (cast `/Game/Characters/Enemies/Blueprints/EnemyPawn_Hostage` _returnvalue
    (:`then`
      (bind _returnvalue_4 (`KismetSystemLibrary.K2_SetTimer` null "SafeZones" 2.0 true))
      (set `self.SafeZone Handle` _returnvalue_4)
      (bind _ascharacter_movement_component (cast `CharacterMovementComponent` (`Pawn.GetMovementComponent` _returnvalue)))
      (`CharacterMovementComponent.SetAvoidanceEnabled` _ascharacter_movement_component true))
    (:`CastFailed`
      _))
  ;[1 1 1] Add Path Nodes
  (bind _outactors_2 (`GameplayStatics.GetAllActorsOfClass` "/Game/Base/Blueprints/ParentSpawnPoint.ParentSpawnPoint_C"))
  (for _array_element_2 _outactors_2
    (`KismetArrayLibrary.Array_Add` (`self.PathingArray`) _array_element_2)))

(event `CheckforPlayer`
  (bind _returnvalue_location (`KismetMathLibrary.BreakTransform` (`self.GetTransform` (`self.K2_GetPawn`))))
  ;[1 1 1] Checks in a 600u Radius for Player Type and Relays Hit Location
  (bind _outhit (`KismetSystemLibrary.CapsuleTraceSingleForObjects` _returnvalue_location _returnvalue_location 800.0 200.0 (`self.TargetPlayer`) false (`|MakeArray` self :!type "Actor Object Reference")))
  (`|ExecutionSequence`
    (:`then_0`
      (bind (_bblockinghit _binitialoverlap _time _distance _location _impactpoint _normal _impactnormal _physmat _hitactor) (`GameplayStatics.BreakHitResult` _outhit))
      (bind _asbp_player_character (cast `/Game/Characters/Player/Blueprints/BP_PlayerCharacter` _hitactor))
      (`self.PlayerLoS` _asbp_player_character))
    (:`then_1`
      (bind _asenemy_pawn_hostage (cast `/Game/Characters/Enemies/Blueprints/EnemyPawn_Hostage` _hitactor))
      (`self.HostageLoS` _asenemy_pawn_hostage))
    (:`then_2`
      (bind _asenemy_pawn_parent (cast `/Game/Characters/Enemies/Blueprints/EnemyPawn_Parent` _hitactor))
      (`self.EnemyLoS` _asenemy_pawn_parent))))

(event `GetNewPath`
  ;[1 1 1] Return Random Path
  (set `self.CurrentPathNode` null)
  (`self.GetStartingPath` (`|GetArrayItem` (`self.PathingArray`) (`KismetMathLibrary.RandomInteger` 4))))

(event `SafeZones`
  (bind _outactors (`GameplayStatics.GetAllActorsOfClass` "/Game/Base/Blueprints/LevelZones.LevelZones_C"))
  (for _array_element _outactors
    (if (`/Game/Base/Blueprints/LevelZones.Safe?` _array_element)
      (set `self.CurrentSafeNode` _array_element)
      (else
        (`KismetSystemLibrary.PrintString` "No Safe Zones")))))

(fn `EnemyLoS`
  (params (Pawn :type "Object Object Reference"))
  (bind _returnvalue_location (`KismetMathLibrary.BreakTransform` (`self.GetTransform` (`self.K2_GetPawn`))))
  (bind _asenemy_pawn_parent (cast `/Game/Characters/Enemies/Blueprints/EnemyPawn_Parent` Pawn)
    (:`then`
      (bind (_outhit _returnvalue) (`KismetSystemLibrary.LineTraceSingleForObjects` _returnvalue_location (`SceneComponent.K2_GetComponentLocation` (`Character.Mesh` _asenemy_pawn_parent)) (`self.Obsticles`)))
      (if _returnvalue
        (set `self.canseePlayer?` false)
        (message `/Game/Characters/Enemies/Blueprints/Int_AIFunc.FollowPathing` (`self.K2_GetPawn`))
        (else
          (set `self.canseePlayer?` true)
          (set `self.EnemyTarget` _asenemy_pawn_parent)
          (message `/Game/Characters/Enemies/Blueprints/Int_AIFunc.ChasePlayer` (`self.K2_GetPawn`)))))
    (:`CastFailed`
      (set `self.canseePlayer?` false)
      (message `/Game/Characters/Enemies/Blueprints/Int_AIFunc.FollowPathing` (`self.K2_GetPawn`)))))

(fn `GetStartingPath`
  (params (`Starting Path` :type "/Game/Base/Blueprints/ParentSpawnPoint Object Reference"))
  ;[1 1 1] Set AI Path Node
  (set `self.CurrentPathNode` `Starting Path`))

(fn `Hostage_Attach`
  (set `self.AttachtoPlayer` true)
  (return))

(fn `HostageLoS`
  (params (Pawn :type "Object Object Reference"))
  (bind _returnvalue_location (`KismetMathLibrary.BreakTransform` (`self.GetTransform` (`self.K2_GetPawn`))))
  ;[1 1 1] Find Hostage Pawn and chace if in LineofSight
  (bind _asenemy_pawn_hostage (cast `/Game/Characters/Enemies/Blueprints/EnemyPawn_Hostage` Pawn)
    (:`then`
      (bind (_outhit _returnvalue) (`KismetSystemLibrary.LineTraceSingleForObjects` _returnvalue_location (`SceneComponent.K2_GetComponentLocation` (`Character.Mesh` _asenemy_pawn_hostage)) (`self.Obsticles`) false (`|MakeArray` self)))
      (if _returnvalue
        (set `self.canseePlayer?` false)
        (message `/Game/Characters/Enemies/Blueprints/Int_AIFunc.FollowPathing` (`self.K2_GetPawn`))
        (else
          (set `self.canseePlayer?` true)
          (set `self.AITarget` _asenemy_pawn_hostage)
          (message `/Game/Characters/Enemies/Blueprints/Int_AIFunc.ChasePlayer` (`self.K2_GetPawn`)))))
    (:`CastFailed`
      (set `self.canseePlayer?` false)
      (message `/Game/Characters/Enemies/Blueprints/Int_AIFunc.FollowPathing` (`self.K2_GetPawn`)))))

(fn `PlayerLoS`
  (params (Pawn :type "Object Object Reference"))
  (bind _returnvalue_location (`KismetMathLibrary.BreakTransform` (`self.GetTransform` (`self.K2_GetPawn`))))
  (bind _asbp_player_character (cast `/Game/Characters/Player/Blueprints/BP_PlayerCharacter` Pawn)
    (:`then`
      (bind (_outhit _returnvalue) (`KismetSystemLibrary.LineTraceSingleForObjects` _returnvalue_location (`SceneComponent.K2_GetComponentLocation` (`Character.Mesh` _asbp_player_character)) (`self.Obsticles`)))
      (if _returnvalue
        (set `self.canseePlayer?` false)
        (message `/Game/Characters/Enemies/Blueprints/Int_AIFunc.FollowPathing` (`self.K2_GetPawn`))
        (else
          (set `self.canseePlayer?` true)
          (set `self.AITarget` _asbp_player_character)
          (message `/Game/Characters/Enemies/Blueprints/Int_AIFunc.ChasePlayer` (`self.K2_GetPawn`)))))
    (:`CastFailed`
      (set `self.canseePlayer?` false)
      (message `/Game/Characters/Enemies/Blueprints/Int_AIFunc.FollowPathing` (`self.K2_GetPawn`)))))

(fn `PossessAIPawns`
  ;[1 1 1] Possess Spawned Pawns
  (bind _outactors (`GameplayStatics.GetAllActorsOfClass` "/Game/Characters/Enemies/Blueprints/EnemyPawn_Parent.EnemyPawn_Parent_C"))
  (for _ _outactors
    (bind _asenemy_pawn_parent (cast `/Game/Characters/Enemies/Blueprints/EnemyPawn_Parent` (`self.K2_GetPawn`)))
    (bind _output_get (set `self.ControlledPawn` _asenemy_pawn_parent))
    (`self.Possess` _output_get)))

(fn `Run_BTs`
  (params (Type :type "/Game/Base/Blueprints/Enum_EnemyTypes Enum" :default "NewEnumerator0"))
  (switch `/Game/Base/Blueprints/Enum_EnemyTypes` Type
    (:`NewEnumerator0`
      (`self.RunBehaviorTree` (`self.BT_RangedRef`)))
    (:`NewEnumerator1`
      (`self.RunBehaviorTree` (`self.BT_MeleeRef`)))
    (:`NewEnumerator2`
      (`self.RunBehaviorTree` (`self.BT_HostageRef`)))))

(fn `UserConstructionScript`)