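; BP_Door is a door actor that moves to a target point when the player character first overlaps its DoorTrig volume.
; The overlap passes a DoOnce with no reset into ActivateDoor, where a timeline lerps the door toward TargetPoint.
; The lerp starts from the current location each update, compounding the curve's alpha.
; Closedoor is called after a delay but is empty, so nothing moves the door back.
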(event `ActivateDoor`
  ;[1 1 1] Move Ship to Target Point Location
  (bind (_direction _movetoalpha) (`Timeline|Timeline_0` :!via `PlayFromStart`)
    (:`Update`
      (`self.K2_SetActorLocation` (`KismetMathLibrary.VLerp` (`self.K2_GetActorLocation`) (`self.K2_GetActorLocation` (`self.TargetPoint`)) _movetoalpha)))))

(event `Closedoor`
  ;[1 1 1] Move Ship to Target Point Location
)

(event `self.DoorTrig.OnComponentBeginOverlap`
  (params (OverlappedComponent :type "PrimitiveComponent Object Reference") (OtherActor :type "Actor Object Reference") (OtherComp :type "PrimitiveComponent Object Reference") (OtherBodyIndex :type Integer) (bFromSweep :type Boolean) (SweepResult :type "HitResult Structure (by ref)"))
  (cast `/Game/Characters/Player/Blueprints/BP_PlayerCharacter` OtherActor)
  (`/Engine/EditorBlueprintResources/StandardMacros.DoOnce` false
    (:`Completed`
      (`self.ActivateDoor`)
      (`KismetSystemLibrary.Delay` 3.0)
      (`self.Closedoor`))))

(fn `UserConstructionScript`)