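; EP_Hostage is an enemy child Blueprint for a hostage character, configured as a variant with a zero attack rate.
; On BeginPlay it runs the parent logic, then copies the melee health and speed values into its total HP and run speed, and sets its type enum.
; Tick and the construction script only call the parent, so all other behavior is inherited.
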(event `self.ReceiveBeginPlay`
  (`parent.ReceiveBeginPlay`)
  (set `self.TotalHP` (`self.MeleeHP`))
  (set `self.AttackRate` 0.0)
  (set `self.RunSpeed` (`self.MeleeSpeed`))
  (set `self.Type` "NewEnumerator2"))

(event `self.ReceiveTick`
  (params (DeltaSeconds :type "Float (single-precision)"))
  (`parent.ReceiveTick` DeltaSeconds))

(fn `UserConstructionScript`
  (`parent.UserConstructionScript`))