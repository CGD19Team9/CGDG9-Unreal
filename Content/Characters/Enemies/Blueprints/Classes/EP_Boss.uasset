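; Boss enemy pawn that copies its HP, fire rate, range and damage settings on BeginPlay, then runs BT_Melee on its AI controller.
; Construction script caches the first BP_BossSpawnManager in the level.
; Attack calls Fire, a hitscan trace that randomly either aims at the AI target or calls Missed for a randomly offset trace.
; Both traces damage BP_PlayerCharacter within MaxRange, so a "miss" can still hit.
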(event `self.ReceiveBeginPlay`
  (`parent.ReceiveBeginPlay`)
  (set `self.TotalHP` (`self.BossHPs`))
  (set `self.AttackRate` (`self.FireRate`))
  (set `self.WeaponRange` (`self.SetWeaponRange`))
  (set `self.WeaponDamage` (`self.SetWeaponDamage`))
  (set `self.MaxRange` 800.0)
  (set `self.inBossRoom` true)
  (set `self.Type` "NewEnumerator6")
  (bind _asaicontroller_parent (cast `/Game/Characters/Enemies/Blueprints/Misc/AIControllerParent` (`self.GetController`)))
  (`AIController.RunBehaviorTree` _asaicontroller_parent "/Game/Characters/Enemies/Blueprints/BehaviourTrees/BT_Melee.BT_Melee"))

(fn `Attack`
  (returns (Range :type Boolean))
  (bind _inrange (`self.Fire`))
  (return _inrange))

(fn `Fire`
  (returns (inRange :type Boolean))
  (bind _asaicontroller_parent (cast `/Game/Characters/Enemies/Blueprints/Misc/AIControllerParent` (`AIBlueprintHelperLibrary.GetAIController` self)))
  (bind _aitarget (`/Game/Characters/Enemies/Blueprints/Misc/AIControllerParent.AITarget` _asaicontroller_parent))
  (`/Engine/EditorBlueprintResources/StandardMacros.IsValid` _aitarget
    (:`Is Valid`
      (if (`self.canAttack?`)
        (if (`KismetMathLibrary.RandomBoolWithWeight` 0.5)
          (bind (_returnvalue_x _returnvalue_y _returnvalue_z) (`KismetMathLibrary.BreakVector` (`SceneComponent.K2_GetComponentLocation` (`Actor.RootComponent` _aitarget))))
          (bind _outhit (`KismetSystemLibrary.LineTraceSingle` (`SceneComponent.K2_GetComponentLocation` (`self.Mesh`)) (`KismetMathLibrary.MakeVector` _returnvalue_x _returnvalue_y (+ _returnvalue_z 50.0)) "TraceTypeQuery3" false (`|MakeArray` self :!type "Actor Object Reference")))
          (bind (_bblockinghit _binitialoverlap _time _distance _location _impactpoint _normal _impactnormal _physmat _hitactor _hitcomponent _hitbonename _hititem _faceindex _tracestart _traceend) (`GameplayStatics.BreakHitResult` _outhit))
          ;[1 1 1] Check Range and Only Apply Damage if in Range
          (if (<= (`KismetMathLibrary.VSize` (- _tracestart _traceend)) (`self.MaxRange`))
            (bind _asbp_player_character (cast `/Game/Characters/Player/Blueprints/BP_PlayerCharacter` _hitactor))
            (`self.ApplyDamage` _asbp_player_character)
            (return true)
            (else
              (return false)))
          (else
            (`self.Missed`)
            (return true)))))))

(fn `Missed`
  (bind _asaicontroller_parent (cast `/Game/Characters/Enemies/Blueprints/Misc/AIControllerParent` (`self.GetController` self)))
  (bind _aitarget (`/Game/Characters/Enemies/Blueprints/Misc/AIControllerParent.AITarget` _asaicontroller_parent))
  (`/Engine/EditorBlueprintResources/StandardMacros.IsValid` _aitarget
    (:`Is Valid`
      (if (`self.canAttack?`)
        (bind (_returnvalue_x _returnvalue_y _returnvalue_z) (`KismetMathLibrary.BreakVector` (`self.K2_GetActorLocation` _aitarget)))
        (bind _outhit (`KismetSystemLibrary.LineTraceSingle` (`SceneComponent.K2_GetComponentLocation` (`self.Mesh`)) (`KismetMathLibrary.MakeVector` (`KismetMathLibrary.RandomFloatInRange` _returnvalue_x (+ _returnvalue_x 120.0)) (`KismetMathLibrary.RandomFloatInRange` _returnvalue_y (+ _returnvalue_y 120.0)) _returnvalue_z) "TraceTypeQuery3" false (`|MakeArray` self :!type "Actor Object Reference")))
        (bind (_bblockinghit _binitialoverlap _time _distance _location _impactpoint _normal _impactnormal _physmat _hitactor _hitcomponent _hitbonename _hititem _faceindex _tracestart _traceend) (`GameplayStatics.BreakHitResult` _outhit))
        (if (<= (`KismetMathLibrary.VSize` (- _tracestart _traceend)) (`self.MaxRange`))
          (bind _asbp_player_character (cast `/Game/Characters/Player/Blueprints/BP_PlayerCharacter` _hitactor))
          (`self.ApplyDamage` _asbp_player_character))))))

(fn `UserConstructionScript`
  (`parent.UserConstructionScript`)
  (bind _outactors (`GameplayStatics.GetAllActorsOfClass` "/Game/Characters/Enemies/Blueprints/Misc/BP_BossSpawnManager.BP_BossSpawnManager_C"))
  (set `self.Manager_Ref` (`|GetArrayItem` _outactors)))