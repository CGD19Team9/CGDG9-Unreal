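; EP_LittleMuscle is an enemy character Blueprint that configures the Little Muscle variant and its weapon attack.
; On BeginPlay, after the parent runs, it copies its own settings for particle, health, attack rate, weapon range and damage into shared variables and sets its type enum.
; Attack damages the first player character overlapping LMWeapon and returns true immediately.
; Tick, overlap and construction add no logic of their own.
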(event `self.ReceiveBeginPlay`
  (`parent.ReceiveBeginPlay`)
  (set `self.UpdatedParticle` (`self.SetParticle`))
  (set `self.TotalHP` (`self.LM_HP`))
  (set `self.AttackRate` (`self.Set Attack Rate`))
  (set `self.WeaponRange` (`self.SetWeaponRange`))
  (set `self.WeaponDamage` (`self.SetWeaponDamage`))
  (set `self.Type` "NewEnumerator1"))

(fn `Attack`
  (returns (Range :type Boolean))
  (for _array_element (`PrimitiveComponent.GetOverlappingActors` (`self.LMWeapon`) "/Game/Characters/Player/Blueprints/BP_PlayerCharacter.BP_PlayerCharacter_C")
    (`GameplayStatics.ApplyDamage` _array_element (`self.WeaponDamage`))
    (return true)))

(fn `UserConstructionScript`
  (`parent.UserConstructionScript`))