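; EP_Undulator is an EP_Parent-derived enemy with a radial area attack that hurts players and enemies alike.
; BeginPlay copies its own health, fire rate, range and damage settings into the parent's stats and sets its type.
; Attack calls Fire, which damages player and enemy hits from a sphere trace around itself.
; The trace uses a fixed radius rather than WeaponRange, does not ignore self, and leaves persistent debug drawing on.
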(event `self.ReceiveBeginPlay`
  (`parent.ReceiveBeginPlay`)
  (set `self.TotalHP` (`self.UndulatorHP`))
  (set `self.AttackRate` (`self.FireRate`))
  (set `self.WeaponRange` (`self.SetWeaponRange`))
  (set `self.WeaponDamage` (`self.SetWeaponDamage`))
  (set `self.Type` "NewEnumerator5"))

(fn `Attack`
  (returns (Range :type Boolean))
  (`self.Fire`)
  (return true))

(fn `Fire`
  (bind _returnvalue (`self.K2_GetActorLocation` self))
  ;[1 1 1] Trace 600u Radius around the pawn and store hits
  (bind _outhits (`KismetSystemLibrary.SphereTraceMultiForObjects` :`Start` _returnvalue :`End` _returnvalue :`Radius` 600.0 :`ObjectTypes` (`self.Targets`) :`DrawDebugType` "Persistent" :`bIgnoreSelf` false))
  (for _array_element _outhits
    (bind (_bblockinghit _binitialoverlap _time _distance _location _impactpoint _normal _impactnormal _physmat _hitactor) (`GameplayStatics.BreakHitResult` _array_element))
    ;[1 1 1] Apply 100 Damage to EnemyPawns and Player Pawns with Radius
    (bind _asbp_player_character (cast `/Game/Characters/Player/Blueprints/BP_PlayerCharacter` _hitactor)
      (:`then`
        (`GameplayStatics.ApplyDamage` _asbp_player_character (`self.WeaponDamage`)))
      (:`CastFailed`
        (bind _asep_parent (cast `/Game/Characters/Enemies/Blueprints/Classes/EP_Parent` _hitactor))
        (`GameplayStatics.ApplyDamage` _asep_parent (`self.WeaponDamage`))))))

(fn `UserConstructionScript`
  (`parent.UserConstructionScript`))