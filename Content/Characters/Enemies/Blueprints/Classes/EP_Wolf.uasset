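; Wolf enemy Blueprint that specializes a parent class with its own health, attack rate, weapon range, damage and enemy type.
; BeginPlay runs the parent logic, then copies the wolf's values into the shared stat variables.
; Attack gathers player characters overlapping the WWeapon component and applies weapon damage after an AttackRate delay placed inside the loop.
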(event `self.ReceiveBeginPlay`
  (`parent.ReceiveBeginPlay`)
  (set `self.TotalHP` (`self.WolfHP`))
  (set `self.AttackRate` (`self.SetAttackRate`))
  (set `self.WeaponRange` (`self.SetWeaponRange`))
  (set `self.WeaponDamage` (`self.SetWeaponDamage`))
  (set `self.Type` "NewEnumerator3"))

(event `/Game/Characters/Enemies/Blueprints/Misc/Int_AIFunc.Attack`
  (for _array_element (`PrimitiveComponent.GetOverlappingActors` (`self.WWeapon`) "/Game/Characters/Player/Blueprints/BP_PlayerCharacter.BP_PlayerCharacter_C")
    (`KismetSystemLibrary.Delay` (`self.AttackRate`))
    (`GameplayStatics.ApplyDamage` _array_element (`self.WeaponDamage`))))

(fn `UserConstructionScript`
  (`parent.UserConstructionScript`))