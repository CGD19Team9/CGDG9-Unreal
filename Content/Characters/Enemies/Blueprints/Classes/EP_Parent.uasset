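; EP_Parent is a base enemy character Blueprint that handles health and attack damage.
; AnyDamage subtracts from TotalHP and calls CheckHP, which runs RemoveActor to destroy the actor at zero or below.
; ApplyDamage deals WeaponDamage to a target only while CanAttack is true.
; ChasePlayer and FollowPathing are empty events, and the walk/run speed changes and softer hide-and-disable removal logic are disconnected.
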(event `self.ReceiveBeginPlay`)

(event `self.ReceiveAnyDamage`
  (params (Damage :type "Float (single-precision)") (DamageType :type "DamageType Object Reference") (InstigatedBy :type "Controller Object Reference") (DamageCauser :type "Actor Object Reference"))
  (bind _totalhp (`self.TotalHP`))
  (`KismetSystemLibrary.PrintString` "damaged")
  (if (<= _totalhp 0.0)
    (`self.CheckHP`)
    (else
      (set `self.TotalHP` (- _totalhp Damage))
      (`self.CheckHP`))))

(event `/Game/Characters/Enemies/Blueprints/Misc/Int_AIFunc.ChasePlayer`)

(event `/Game/Characters/Enemies/Blueprints/Misc/Int_AIFunc.FollowPathing`)

(fn `ApplyDamage`
  (params (TargettedActor :type "/Game/Characters/Player/Blueprints/BP_PlayerCharacter Object Reference"))
  ;[1 1 1] Apply Damage to Target
  (if (`self.canAttack?`)
    (`GameplayStatics.ApplyDamage` TargettedActor (`self.WeaponDamage`) null self)
    (else
      (`KismetSystemLibrary.PrintString` "can't atttack"))))

(fn `CheckHP`
  (if (<= (`self.TotalHP`) 0.0)
    (`self.RemoveActor`)))

(fn `RemoveActor`
  ;[1 1 1] Hide EnemyAI, check cannot attack and invalidate damage raduis
  (`self.K2_DestroyActor`))

(fn `UserConstructionScript`)