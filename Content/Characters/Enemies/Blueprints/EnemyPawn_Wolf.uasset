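; Wolf enemy pawn, a child Blueprint that configures inherited enemy behavior as a short-range variant using the melee health and speed values.
; On BeginPlay it runs the parent logic, then sets total HP, attack rate, run speed, weapon range and enemy type.
; It adds no other logic: the construction script only calls the parent, and the overlap and tick events are disabled.
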(event `self.ReceiveBeginPlay`
  (`parent.ReceiveBeginPlay`)
  (set `self.TotalHP` (`self.MeleeHP`))
  (set `self.AttackRate` 0.8)
  (set `self.RunSpeed` (`self.MeleeSpeed`))
  (set `self.WeaponRange` 5.0)
  (set `self.Type` "NewEnumerator3"))

(fn `UserConstructionScript`
  (`parent.UserConstructionScript`))