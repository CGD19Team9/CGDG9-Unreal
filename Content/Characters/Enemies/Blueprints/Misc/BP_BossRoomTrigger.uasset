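; BP_BossRoomTrigger is an overlap volume that starts the boss spawn when the player character enters it.
; If spawning is allowed, it fires once, calling CallSpawnBoss on the first BP_BossSpawnManager found in the level.
; After a short delay, it disables spawning on every BP_BossRoomTrigger and switches their TriggerPoint collision to block all channels, turning the triggers into barriers.
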(event `self.TriggerPoint.OnComponentBeginOverlap`
  (params (OverlappedComponent :type "PrimitiveComponent Object Reference") (OtherActor :type "Actor Object Reference") (OtherComp :type "PrimitiveComponent Object Reference") (OtherBodyIndex :type Integer) (bFromSweep :type Boolean) (SweepResult :type "HitResult Structure (by ref)"))
  (bind _outactors (`GameplayStatics.GetAllActorsOfClass` "/Game/Characters/Enemies/Blueprints/Misc/BP_BossSpawnManager.BP_BossSpawnManager_C"))
  (cast `/Game/Characters/Player/Blueprints/BP_PlayerCharacter` OtherActor)
  (if (`self.canSpawnBoss`)
    (`/Engine/EditorBlueprintResources/StandardMacros.DoOnce` false
      (:`Completed`
        (`/Game/Characters/Enemies/Blueprints/Misc/BP_BossSpawnManager.SpawnBoss` (`|GetArrayItem` _outactors))
        (`KismetSystemLibrary.Delay` 1.5)
        (bind _outactors_2 (`GameplayStatics.GetAllActorsOfClass` "BP_BossRoomTrigger_C"))
        (for _array_element _outactors_2
          (set `/Game/Characters/Enemies/Blueprints/Misc/BP_BossRoomTrigger.canSpawnBoss` false _array_element))
        (bind _outactors_3 (`GameplayStatics.GetAllActorsOfClass` "BP_BossRoomTrigger_C"))
        (for _array_element_2 _outactors_3
          (`PrimitiveComponent.SetCollisionResponseToAllChannels` (`/Game/Characters/Enemies/Blueprints/Misc/BP_BossRoomTrigger.TriggerPoint` _array_element_2) "ECR_Block"))))))

(fn `UserConstructionScript`)