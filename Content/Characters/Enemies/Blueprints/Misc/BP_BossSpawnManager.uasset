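; Boss room spawn manager that spawns EP_Boss and three one-shot waves of minions through bound events.
; The construction script gathers the boss spawn point, minion points and room triggers.
; Each point's per-wave enemy type feeds an enum switch to class-specific spawners, which flag minions as in the boss room and count them.
; AIDestroyed lowers that count and re-enables AbletoSpawn, which gates waves two and three.
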(event `self.ReceiveBeginPlay`
  ;[1 1 1] Spawn "EP_Boss" at Boss Spawn Point
  (add `self.SpawnBoss` (delegate `SpawnBoss_Event`))
  ;[1 1 1] Spawn First AI Wave
  (add `self.SpawnWave_1` (delegate `SpawnWave_1_Event`))
  ;[1 1 1] Spawn Second AI Wave
  (add `self.SpawnWave_2` (delegate `SpawnWave_2_Event`))
  ;[1 1 1] Spawn Third AI Wave
  (add `self.SpawnWave_3` (delegate `SpawnWave_3_Event`)))

(event `SpawnWave_2_Event`
  ;[1 1 1] Spawn Second AI Wave
  (`/Engine/EditorBlueprintResources/StandardMacros.DoOnce` false
    (:`Completed`
      (if (`self.AbletoSpawn`)
        (for _array_element (`self.MinionPoints`)
          (`self.AIClass_Switch` (`/Game/Characters/Enemies/Blueprints/Misc/BP_BossRoomSpawns.SW_SpawnType` _array_element) (`self.K2_GetActorLocation` _array_element) (`self.K2_GetActorRotation` _array_element))
          (set `self.AbletoSpawn` false))))))

(event `SpawnBoss_Event`
  (bind _bossspawnpoint (`self.BossSpawnPoint`))
  ;[1 1 1] Spawn "EP_Boss" at Boss Spawn Point
  (bind _returnvalue (`AIBlueprintHelperLibrary.SpawnAIFromClass` "/Game/Characters/Enemies/Blueprints/Classes/EP_Boss.EP_Boss_C" "/Game/Characters/Enemies/Blueprints/BehaviourTrees/BT_Ranged.BT_Ranged" (`self.K2_GetActorLocation` _bossspawnpoint) (`self.K2_GetActorRotation` _bossspawnpoint)))
  (bind _asep_boss (cast `/Game/Characters/Enemies/Blueprints/Classes/EP_Boss` _returnvalue))
  (set `self.Boss` _asep_boss))

(event `SpawnWave_1_Event`
  ;[1 1 1] Spawn First AI Wave
  (`/Engine/EditorBlueprintResources/StandardMacros.DoOnce` false
    (:`Completed`
      (for _array_element (`self.MinionPoints`)
        (`self.AIClass_Switch` (`/Game/Characters/Enemies/Blueprints/Misc/BP_BossRoomSpawns.FW_SpawnType` _array_element) (`self.K2_GetActorLocation` _array_element) (`self.K2_GetActorRotation` _array_element))))))

(event `SpawnWave_3_Event`
  ;[1 1 1] Spawn Third AI Wave
  (`/Engine/EditorBlueprintResources/StandardMacros.DoOnce` false
    (:`Completed`
      (if (`self.AbletoSpawn`)
        (for _array_element (`self.MinionPoints`)
          (`self.AIClass_Switch` (`/Game/Characters/Enemies/Blueprints/Misc/BP_BossRoomSpawns.TW_SpawnType` _array_element) (`self.K2_GetActorLocation` _array_element) (`self.K2_GetActorRotation` _array_element))
          (set `self.AbletoSpawn` false))))))

(fn `AI_Destroyed`
  ;[1 1 1] When all AI is Destroyed set "AbletoSpawn" to True for next Wave
  (bind _result (`/Engine/EditorBlueprintResources/StandardMacros.DecrementFloat` (`self.AliveAI`))
    (:`  `
      (if (<= _result 1.0)
        (set `self.AbletoSpawn` true)))))

(fn `AIClass_Switch`
  (params (Type :type "/Game/Base/Blueprints/Enum_EnemyTypes Enum" :default "NewEnumerator0") (Location :type "Vector Structure") (Rotation :type "Rotator Structure"))
  ;[1 1 1] Spawn AI Class on Enum_EnemyTypes
  (switch `/Game/Base/Blueprints/Enum_EnemyTypes` Type
    (:`NewEnumerator0`
      (`self.Spawn_Muscles` Location Rotation))
    (:`NewEnumerator1`
      (`self.Spawn_LittleMuscles` Location Rotation))
    (:`NewEnumerator3`
      (`self.Spawn_Wolves` Location Rotation))
    (:`NewEnumerator4`
      (`self.Spawn_Gremlins` Location Rotation))
    (:`NewEnumerator5`
      (`self.Spawn_Undulators` Location Rotation))))

(fn `Spawn_Gremlins`
  (params (Location :type "Vector Structure") (Rotation :type "Rotator Structure"))
  (bind _returnvalue (`AIBlueprintHelperLibrary.SpawnAIFromClass` "/Game/Characters/Enemies/Blueprints/Classes/EP_Gremlin.EP_Gremlin_C" "/Game/Characters/Enemies/Blueprints/BehaviourTrees/BT_Ranged.BT_Ranged" Location Rotation))
  (bind _asep_parent (cast `/Game/Characters/Enemies/Blueprints/Classes/EP_Parent` _returnvalue))
  (set `/Game/Characters/Enemies/Blueprints/Classes/EP_Parent.inBossRoom` true _asep_parent)
  (`/Engine/EditorBlueprintResources/StandardMacros.IncrementFloat` (`self.AliveAI`)))

(fn `Spawn_LittleMuscles`
  (params (Location :type "Vector Structure") (Rotation :type "Rotator Structure"))
  ;[1 1 1] Spawn AI of Class at Spawn Point. Update "inBossRoom" Bool and Increment to "AliveAI" Float
  (`/Engine/EditorBlueprintResources/StandardMacros.DoOnce` false
    (:`Completed`
      (bind _returnvalue (`AIBlueprintHelperLibrary.SpawnAIFromClass` "/Game/Characters/Enemies/Blueprints/Classes/EP_LittleMuscle.EP_LittleMuscle_C" "/Game/Characters/Enemies/Blueprints/BehaviourTrees/BT_Melee.BT_Melee" Location Rotation))
      (bind _asep_parent (cast `/Game/Characters/Enemies/Blueprints/Classes/EP_Parent` _returnvalue))
      (set `/Game/Characters/Enemies/Blueprints/Classes/EP_Parent.inBossRoom` true _asep_parent)
      (`/Engine/EditorBlueprintResources/StandardMacros.IncrementFloat` (`self.AliveAI`)))))

(fn `Spawn_Muscles`
  (params (Location :type "Vector Structure") (Rotation :type "Rotator Structure"))
  (bind _returnvalue (`AIBlueprintHelperLibrary.SpawnAIFromClass` "/Game/Characters/Enemies/Blueprints/Classes/EP_Muscle.EP_Muscle_C" "/Game/Characters/Enemies/Blueprints/BehaviourTrees/BT_Ranged.BT_Ranged" Location Rotation))
  (bind _asep_parent (cast `/Game/Characters/Enemies/Blueprints/Classes/EP_Parent` _returnvalue))
  (set `/Game/Characters/Enemies/Blueprints/Classes/EP_Parent.inBossRoom` true _asep_parent)
  (`/Engine/EditorBlueprintResources/StandardMacros.IncrementFloat` (`self.AliveAI`)))

(fn `Spawn_Undulators`
  (params (Location :type "Vector Structure") (Rotation :type "Rotator Structure"))
  (bind _returnvalue (`AIBlueprintHelperLibrary.SpawnAIFromClass` "/Game/Characters/Enemies/Blueprints/Classes/EP_Undulator.EP_Undulator_C" "/Game/Characters/Enemies/Blueprints/BehaviourTrees/BT_Melee.BT_Melee" Location Rotation))
  (bind _asep_parent (cast `/Game/Characters/Enemies/Blueprints/Classes/EP_Parent` _returnvalue))
  (set `/Game/Characters/Enemies/Blueprints/Classes/EP_Parent.inBossRoom` true _asep_parent)
  (`/Engine/EditorBlueprintResources/StandardMacros.IncrementFloat` (`self.AliveAI`)))

(fn `Spawn_Wolves`
  (params (Location :type "Vector Structure") (Rotation :type "Rotator Structure"))
  (bind _returnvalue (`AIBlueprintHelperLibrary.SpawnAIFromClass` "/Game/Characters/Enemies/Blueprints/Classes/EP_Wolf.EP_Wolf_C" "/Game/Characters/Enemies/Blueprints/BehaviourTrees/BT_Melee.BT_Melee" Location Rotation))
  (bind _asep_parent (cast `/Game/Characters/Enemies/Blueprints/Classes/EP_Parent` _returnvalue))
  (set `/Game/Characters/Enemies/Blueprints/Classes/EP_Parent.inBossRoom` true _asep_parent)
  (`/Engine/EditorBlueprintResources/StandardMacros.IncrementFloat` (`self.AliveAI`)))

(fn `UserConstructionScript`
  (bind _outactors (`GameplayStatics.GetAllActorsOfClass` "/Game/Characters/Enemies/Blueprints/Misc/BP_BossSpawnPoint.BP_BossSpawnPoint_C"))
  (set `self.BossSpawnPoint` (`|GetArrayItem` _outactors))
  (bind _outactors_2 (`GameplayStatics.GetAllActorsOfClass` "/Game/Characters/Enemies/Blueprints/Misc/BP_BossRoomSpawns.BP_BossRoomSpawns_C"))
  (for _array_element _outactors_2
    (`KismetArrayLibrary.Array_Add` (`self.MinionPoints`) _array_element))
  (bind _outactors_3 (`GameplayStatics.GetAllActorsOfClass` "/Game/Characters/Enemies/Blueprints/Misc/BP_BossRoomTrigger.BP_BossRoomTrigger_C"))
  (for _array_element_2 _outactors_3
    (`KismetArrayLibrary.Array_Add` (`self.BossSpawnWalls`) _array_element_2)))