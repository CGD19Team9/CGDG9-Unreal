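; Parent AI controller for EP_Parent enemies, handling awareness of the player and other enemies plus waypoint selection.
; A looping timer capsule-traces within the pawn's weapon range, then line-traces against obstacles for line of sight.
; Results set targets and message the pawn to chase or follow its path.
; Waypoints are gathered at BeginPlay for a delayed random pick, while another timer tracks a safe level zone.
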(event `self.ReceiveBeginPlay`
  ;[1 1 1] Possess Pawns on Spawn and Run AI Awareness
  (bind _returnvalue (`KismetSystemLibrary.K2_SetTimer` null "CheckforPlayer" 0.1 true))
  (set `self.AIPerceptionHandle` _returnvalue)
  (bind _returnvalue_2 (`KismetSystemLibrary.K2_SetTimer` null "GetNewPath" 2.0))
  (set `self.PathingTimerHandle` _returnvalue_2)
  (bind _returnvalue_3 (`KismetSystemLibrary.K2_SetTimer` null "SafeZones" 2.0 true))
  (set `self.SafeZone Handle` _returnvalue_3)
  ;[1 1 1] Add Path Nodes
  (bind _outactors (`GameplayStatics.GetAllActorsOfClass` "/Game/Characters/Enemies/Blueprints/Misc/Waypoints.Waypoints_C"))
  (for _array_element _outactors
    (`KismetArrayLibrary.Array_Add` (`self.PathingArray`) _array_element)))

(event `CheckforPlayer`
  (bind _returnvalue (`self.K2_GetPawn`))
  (bind _returnvalue_location (`KismetMathLibrary.BreakTransform` (`self.GetTransform` _returnvalue)))
  ;[1 1 1] Checks in a 800u Radius for Player, Hostage and Enemy Type and Relays Hit Location
  (bind _asep_parent (cast `/Game/Characters/Enemies/Blueprints/Classes/EP_Parent` _returnvalue))
  (bind _outhits (`KismetSystemLibrary.CapsuleTraceMultiForObjects` _returnvalue_location _returnvalue_location (`/Game/Characters/Enemies/Blueprints/Classes/EP_Parent.WeaponRange` _asep_parent) 400.0 (`self.TargetPlayer`) false (`|MakeArray` self :!type "Actor Object Reference")))
  (set `self.canseePlayer?` false)
  (for _array_element _outhits
    (`|ExecutionSequence`
      (:`then_0`
        (bind (_bblockinghit _binitialoverlap _time _distance _location _impactpoint _normal _impactnormal _physmat _hitactor) (`GameplayStatics.BreakHitResult` _array_element))
        (bind _asbp_player_character (cast `/Game/Characters/Player/Blueprints/BP_PlayerCharacter` _hitactor))
        (`self.PlayerLoS` _asbp_player_character))
      (:`then_1`
        (bind _asep_parent_2 (cast `/Game/Characters/Enemies/Blueprints/Classes/EP_Parent` _hitactor))
        (`self.EnemyLoS` _asep_parent_2)))))

(event `SafeZones`
  (bind _outactors (`GameplayStatics.GetAllActorsOfClass` "/Game/Base/Blueprints/LevelZones.LevelZones_C"))
  (for _array_element _outactors
    (if (`/Game/Base/Blueprints/LevelZones.Safe?` _array_element)
      (set `self.CurrentSafeNode` _array_element))))

(fn `EnemyLoS`
  (params (Pawn :type "Object Object Reference"))
  (bind _returnvalue_location (`KismetMathLibrary.BreakTransform` (`self.GetTransform` (`self.K2_GetPawn`))))
  (bind _asep_parent (cast `/Game/Characters/Enemies/Blueprints/Classes/EP_Parent` Pawn)
    (:`then`
      (bind (_outhit _returnvalue) (`KismetSystemLibrary.LineTraceSingleForObjects` _returnvalue_location (`SceneComponent.K2_GetComponentLocation` (`Character.Mesh` _asep_parent)) (`self.Obsticles`)))
      (if _returnvalue
        (set `self.canseePlayer?` false)
        (message `/Game/Characters/Enemies/Blueprints/Misc/Int_AIFunc.FollowPathing` (`self.K2_GetPawn`))
        (else
          (set `self.canseePlayer?` true)
          (set `self.EnemyTarget` _asep_parent)
          (message `/Game/Characters/Enemies/Blueprints/Misc/Int_AIFunc.ChasePlayer` (`self.K2_GetPawn`)))))
    (:`CastFailed`
      (set `self.canseePlayer?` false)
      (message `/Game/Characters/Enemies/Blueprints/Misc/Int_AIFunc.FollowPathing` (`self.K2_GetPawn`)))))

(fn `GetNewPath`
  (returns (PathPoint :type "/Game/Characters/Enemies/Blueprints/Misc/Waypoints Object Reference"))
  (bind _pathingarray (`self.PathingArray`))
  (bind _output (`|GetArrayItem` _pathingarray (`KismetMathLibrary.RandomInteger` (`KismetArrayLibrary.Array_Length` _pathingarray))))
  (`self.GetStartingPath` _output)
  (return _output))

(fn `GetStartingPath`
  (params (`Starting Path` :type "/Game/Characters/Enemies/Blueprints/Misc/Waypoints Object Reference"))
  ;[1 1 1] Set AI Path Node
  (set `self.CurrentPathNode` `Starting Path`))

(fn `Hostage_Attach`
  ;[1 1 1] Attach Player to Hostage
  (set `self.AttachtoPlayer` true)
  (return))

(fn `PlayerLoS`
  (params (Pawn :type "Object Object Reference"))
  (bind _returnvalue_location (`KismetMathLibrary.BreakTransform` (`self.GetTransform` (`self.K2_GetPawn`))))
  (bind _asbp_player_character (cast `/Game/Characters/Player/Blueprints/BP_PlayerCharacter` Pawn)
    (:`then`
      (bind (_outhit _returnvalue) (`KismetSystemLibrary.LineTraceSingleForObjects` _returnvalue_location (`SceneComponent.K2_GetComponentLocation` (`Character.Mesh` _asbp_player_character)) (`self.Obsticles`) false (`|MakeArray` self :!type "Actor Object Reference")))
      (if _returnvalue
        (set `self.canseePlayer?` false)
        (set `self.AITarget` null)
        (message `/Game/Characters/Enemies/Blueprints/Misc/Int_AIFunc.FollowPathing` (`self.K2_GetPawn`))
        (else
          (set `self.canseePlayer?` true)
          (set `self.AITarget` _asbp_player_character)
          (message `/Game/Characters/Enemies/Blueprints/Misc/Int_AIFunc.ChasePlayer` (`self.K2_GetPawn`)))))
    (:`CastFailed`
      (set `self.canseePlayer?` false)
      (message `/Game/Characters/Enemies/Blueprints/Misc/Int_AIFunc.FollowPathing` (`self.K2_GetPawn`)))))

(fn `PossessAIPawns`
  ;[1 1 1] Possess Spawned Pawns
  (bind _outactors (`GameplayStatics.GetAllActorsOfClass` "/Game/Characters/Enemies/Blueprints/Classes/EP_Parent.EP_Parent_C"))
  (for _ _outactors
    (bind _asep_parent (cast `/Game/Characters/Enemies/Blueprints/Classes/EP_Parent` (`self.K2_GetPawn`)))
    (bind _output_get (set `self.ControlledPawn` _asep_parent))
    (`self.Possess` _output_get)))

(fn `UserConstructionScript`)