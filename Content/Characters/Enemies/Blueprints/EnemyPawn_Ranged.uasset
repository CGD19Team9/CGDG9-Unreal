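; Ranged enemy pawn that shoots at the player with hitscan fire, overriding the parent's range, damage, speed and type on BeginPlay.
; The Attack interface event fires immediately and starts a looping timer on Fire at FireRate.
; When CanAttack and the AI controller's target is valid, Fire traces a custom channel from the mesh to above the target, calling ApplyDamage on player hits.
; Persistent trace drawing and debug prints remain enabled.
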(event `/Game/Characters/Enemies/Blueprints/Int_AIFunc.Attack`
  ;[1 1 1] Call Attack Function from Int_AIFunctions
  (bind _returnvalue (`KismetSystemLibrary.K2_SetTimer` null "Fire" (`self.FireRate`) true))
  (set `self.FireRateHandle` _returnvalue)
  (`self.Fire`))

(event `self.ReceiveBeginPlay`
  ;[1 1 1] Reset Variables from Parent Class
  (`parent.ReceiveBeginPlay`)
  (set `self.WeaponRange` 300.0)
  (set `self.MeleeDamage` 10.0)
  (set `self.RunSpeed` (`self.SetMovement_Ranged`))
  (set `self.Type` "NewEnumerator0"))

(fn `Fire`
  ;[1 1 1] Check if controller target is valid, then line trace through custom channel at target pawn (+50 Z Axis)
  (bind _asaicontroller_parent (cast `/Game/Characters/Enemies/Blueprints/AIControllerParent` (`AIBlueprintHelperLibrary.GetAIController` self)))
  (bind _aitarget (`/Game/Characters/Enemies/Blueprints/AIControllerParent.AITarget` _asaicontroller_parent))
  (`/Engine/EditorBlueprintResources/StandardMacros.IsValid` _aitarget
    (:`Is Valid`
      (if (`self.canAttack?`)
        (bind (_returnvalue_x _returnvalue_y _returnvalue_z) (`KismetMathLibrary.BreakVector` (`SceneComponent.K2_GetComponentLocation` (`Actor.RootComponent` _aitarget))))
        (bind _outhit (`KismetSystemLibrary.LineTraceSingle` (`SceneComponent.K2_GetComponentLocation` (`self.Mesh`)) (`KismetMathLibrary.MakeVector` _returnvalue_x _returnvalue_y (+ _returnvalue_z 50.0)) "TraceTypeQuery3" false (`|MakeArray` self :!type "Actor Object Reference") "Persistent"))
        ;[1 1 1] Check hit result is player then apply damage
        (bind _asbp_player_character (cast `/Game/Characters/Player/Blueprints/BP_PlayerCharacter` (`.HitActor` (`GameplayStatics.BreakHitResult` _outhit)))
          (:`then`
            (`self.ApplyDamage` _asbp_player_character))
          (:`CastFailed`
            (`KismetSystemLibrary.PrintString` "Not PC")))
        (else
          (`KismetSystemLibrary.PrintString` "cantattack"))))))

(fn `UserConstructionScript`
  (`parent.UserConstructionScript`))