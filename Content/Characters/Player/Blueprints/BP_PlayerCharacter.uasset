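; Top-down shooter player character with camera-relative movement, mouse aiming, sprint, combat roll, shields, health and death.
; Tick sets facing toward mouse or velocity, and walk speed from aim and sprint state.
; Looping timers regenerate and drain stamina; rolls spend it, lerping position on a timeline while blocking damage and movement input.
; BPInventory handles pickups and weapon scrolling, feeding a child-actor weapon controlled by interface messages for fire, reload and aim.
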(event `self.ReceiveAnyDamage`
  (params (Damage :type "Float (single-precision)") (DamageType :type "DamageType Object Reference") (InstigatedBy :type "Controller Object Reference") (DamageCauser :type "Actor Object Reference"))
  ;[1 1 1] Damage
  (if (`self.Rolling`)
    _
    (elif (<= (`self.Shields`) 0.0)
      (bind _output_get (set `self.Health` (- (`self.Health`) Damage)))
      (`self.CheckHP` _output_get)
      (else
        (set `self.Shields` (- (`self.Shields`) Damage))))))

(event `self.ReceiveBeginPlay`
  ;[1 1 1] Setup
  (`SceneComponent.K2_SetWorldRotation` (`self.SpringArm`) (`KismetMathLibrary.MakeRotator` 0.0 -60.0 (+ (`self.CameraAngle`) 90.0)) false false)
  (set `self.Health` (`self.MaxHealth`))
  (`self.RegenStamina`))

(event `/Game/Characters/Player/Blueprints/CharacterControllerInterface.WeaponScrollDown`
  ;[1 1 1] Weapon Scroll
  (bind _weapon (`/Game/Characters/Player/Blueprints/Inventory/BP_Inventory.ScrollWeapon` (`self.BP_Inventory`) 1))
  (`KismetSystemLibrary.PrintString` (`KismetSystemLibrary.GetClassDisplayName` _weapon))
  (`ChildActorComponent.SetChildActorClass` (`self.WeaponMountPoint`) _weapon)
  (bind (_value _found) (`/Game/Characters/Player/Blueprints/Inventory/BP_Inventory.GetClip` (`self.BP_Inventory`) (`ChildActorComponent.ChildActorClass` (`self.WeaponMountPoint`)) :!label _label))
  (message `/Game/Weapons/Blueprints/WeaponInterface.SetClip` (`ChildActorComponent.ChildActor` (`self.WeaponMountPoint`)) _value _found))

(event `self.ReceiveTick`
  (params (DeltaSeconds :type "Float (single-precision)"))
  ;[1 1 1] Tick
  (`self.UpdateCharacterRotation`)
  (`self.UpdateMovementSpeed`))

(event `/Game/Characters/Player/Blueprints/CharacterControllerInterface.WeaponScrollUp`
  ;[1 1 1] Weapon Scroll
  (bind _weapon (`/Game/Characters/Player/Blueprints/Inventory/BP_Inventory.ScrollWeapon` (`self.BP_Inventory`) -1))
  (`KismetSystemLibrary.PrintString` (`KismetSystemLibrary.GetClassDisplayName` _weapon))
  (`ChildActorComponent.SetChildActorClass` (`self.WeaponMountPoint`) _weapon)
  (goto _label))

(event `/Game/Characters/Player/Blueprints/CharacterControllerInterface.MoveUp`
  (params (Axis :type "Float (single-precision)"))
  ;[1 1 1] Walking
  (if (`self.Rolling`)
    _
    (elif (!= Axis 0.0)
      (`PawnMovementComponent.AddInputVector` (`self.CharacterMovement`) (`KismetMathLibrary.GreaterGreater_VectorRotator` (* (0.0 1.0 0.0) Axis) (`KismetMathLibrary.MakeRotator` 0.0 0.0 (`self.CameraAngle`))) false))))

(event `RegenStamina`
  ;[1 1 1] Stamina Regen
  (`KismetSystemLibrary.K2_SetTimerDelegate` (delegate `RegenStamina`) (`self.StamRegenTime`) true)
  (if (< (`self.Stamina`) (`self.MaxStamina`))
    (`/Engine/EditorBlueprintResources/StandardMacros.IncrementFloat` (`self.Stamina`))))

(event `/Game/Characters/Player/Blueprints/CharacterControllerInterface.Aiming`
  (params (Aiming :type Boolean))
  ;[1 1 1] Aiming Toggle
  (`|ExecutionSequence`
    (:`then_0`
      (bind _output_get (set `self.Aiming?` Aiming))
      (if _output_get
        (`self.StopSprint`)))
    (:`then_1`
      (message `/Game/Weapons/Blueprints/WeaponInterface.Aiming` (`ChildActorComponent.ChildActor` (`self.WeaponMountPoint`)) Aiming))))

(event `/Game/Characters/Player/Blueprints/CharacterControllerInterface.MoveRight`
  (params (Axis :type "Float (single-precision)"))
  ;[1 1 1] Walking
  (if (`self.Rolling`)
    _
    (elif (!= Axis 0.0)
      (`PawnMovementComponent.AddInputVector` (`self.CharacterMovement`) (`KismetMathLibrary.GreaterGreater_VectorRotator` (* (1.0 0.0 0.0) Axis) (`KismetMathLibrary.MakeRotator` 0.0 0.0 (`self.CameraAngle`))) false))))

(event `/Game/Characters/Player/Blueprints/CharacterControllerInterface.FireGun`
  ;[1 1 1] Fire
  (message `/Game/Weapons/Blueprints/WeaponInterface.FireWeapon` (`ChildActorComponent.ChildActor` (`self.WeaponMountPoint`)) (`self.BP_Inventory`)))

(event `/Game/Characters/Player/Blueprints/CharacterControllerInterface.Sprint`
  (params (Sprinting :type Boolean))
  ;[1 1 1] Sprint
  (if (and Sprinting (not (`self.Aiming?`)))
    (`self.StartSprint`)
    (else
      (`KismetSystemLibrary.K2_ClearAndInvalidateTimerHandle` (`self.StamTimer`) :!label _label_2)
      (set `self.Sprinting` false))))

(event `/Game/Characters/Player/Blueprints/CharacterControllerInterface.InterfaceReload`
  ;[1 1 1] Reload
  (message `/Game/Weapons/Blueprints/WeaponInterface.ManualReload` (`ChildActorComponent.ChildActor` (`self.WeaponMountPoint`)) (`self.BP_Inventory`)))

(event `StopSprint`
  ;[1 1 1] Sprint
  (goto _label_2))

(event `StartSprint`
  ;[1 1 1] Sprint Timer
  (bind _returnvalue (`KismetSystemLibrary.K2_SetTimerDelegate` (delegate `StartSprint`) 0.01 true))
  (set `self.StamTimer` _returnvalue)
  (if (>= (`self.Stamina`) 1.0)
    (set `self.Sprinting` true)
    (`/Engine/EditorBlueprintResources/StandardMacros.DecrementFloat` (`self.Stamina`))
    (else
      (set `self.Sprinting` false))))

(event `/Game/Characters/Player/Blueprints/CharacterControllerInterface.CombatRoll`
  (params (Direction :type "/Game/Characters/Player/Blueprints/Direction Enum" :default "NewEnumerator0"))
  ;[1 1 1] Rolling
  (if (>= (`self.Stamina`) (`self.RollCost`))
    (`/Engine/EditorBlueprintResources/StandardMacros.DoOnce` false :!label _label_3
      (:`Completed`
        (set `self.Stamina` (- (`self.Stamina`) (`self.RollCost`)))
        (set `self.Rolling` true)
        (bind (_start _end) (`self.GetStartAndEnd` Direction))
        (bind (_direction _rollprogress) (`Timeline|Timeline_1` :!via `PlayFromStart`)
          (:`Update`
            (`self.K2_SetActorLocation` (+ (`KismetMathLibrary.VLerp` _start _end _rollprogress) (0.0 0.0 80.0)) true))
          (:`Finished`
            (set `self.Rolling` false)
            (goto _label_3 :!via `Reset`)))))))

(fn `CheckHP`
  (params (Health :type "Float (double-precision)"))
  ;[1 1 1] Checks if HP have reached <=0
  (if (<= Health 0.0)
    (`self.Death`)))

(fn `Death`
  (bind _playercontroller (`self.PlayerController`))
  ;[1 1 1] Hides Player, Disables Input and displays death text
  (`SceneComponent.SetVisibility` (`self.CapsuleComponent`) false false)
  (`SceneComponent.SetVisibility` (`self.Mesh`) false false)
  (`SceneComponent.SetVisibility` (`self.WeaponMountPoint`) false false)
  (`self.DisableInput` _playercontroller)
  (set `/Game/Characters/Player/Blueprints/BP_PlayerController.canMove?` false _playercontroller)
  (`Widget.SetVisibility` (`/Game/Characters/Player/Blueprints/DevHUD.DeathTxt` (`self.UI_Widget`)) "Visible"))

(fn `GetAmmoType`)

(fn `GetStartAndEnd`
  (params (Index :type "/Game/Characters/Player/Blueprints/Direction Enum" :default "NewEnumerator0"))
  (returns (Start :type "Vector Structure") (End :type "Vector Structure"))
  (bind _returnvalue (`SceneComponent.K2_GetComponentLocation` (`self.Mesh`)))
  (return _returnvalue (- _returnvalue (`KismetMathLibrary.GreaterGreater_VectorRotator` (select `/Game/Characters/Player/Blueprints/Direction` Index :`NewEnumerator0` (0.0 -250.0 0.0) :`NewEnumerator1` (0.0 250.0 0.0) :`NewEnumerator2` (-250.0 0.0 0.0) :`NewEnumerator3` (250.0 0.0 0.0) :!type "Vector Structure") (`KismetMathLibrary.MakeRotator` 0.0 0.0 (`self.CameraAngle`))))))

(fn `PickupHealth`
  (params (BaseHealth :type "Float (double-precision)"))
  (returns (Success :type Boolean))
  (bind _returnvalue (+ BaseHealth (`self.Health`)))
  (set `self.Health` (select `bool` (> _returnvalue (`self.MaxHealth`)) :`false` _returnvalue :`true` (`self.MaxHealth`)))
  (return true))

(fn `PickupItem`
  (params (PickupType :type "/Game/Characters/Player/Blueprints/Inventory/PickupType Enum" :default "NewEnumerator0") (AmmoType :type "/Game/Characters/Player/Blueprints/Inventory/AmmoType Enum" :default "NewEnumerator0") (Count :type Integer) (WeaponClass :type "Actor Class Reference"))
  (returns (Success :type Boolean))
  (`/Game/Characters/Player/Blueprints/Inventory/BP_Inventory.AddToInventory` (`self.BP_Inventory`) PickupType AmmoType Count WeaponClass)
  (return true))

(fn `PickupShield`
  (params (BaseShield :type "Float (double-precision)"))
  (returns (Success :type Boolean))
  (bind _returnvalue (+ BaseShield (`self.Shields`)))
  (set `self.Shields` (select `bool` (> _returnvalue (`self.MaxShields`)) :`false` _returnvalue :`true` (`self.MaxShields`)))
  (return true))

(fn `UpdateCharacterRotation`
  (bind (_returnvalue_roll _returnvalue_pitch _returnvalue_yaw) (`KismetMathLibrary.BreakRotator` (`KismetMathLibrary.FindLookAtRotation` (`self.K2_GetActorLocation`) (`self.MouseLocation`))))
  (bind _velocity (`MovementComponent.Velocity` (`self.CharacterMovement`)))
  (bind (_returnvalue_roll_2 _returnvalue_pitch_2 _returnvalue_yaw_2) (`KismetMathLibrary.BreakRotator` (`KismetMathLibrary.MakeRotFromX` _velocity)))
  (`SceneComponent.K2_SetRelativeRotation` (`self.CapsuleComponent`) (select `bool` (or (== _velocity (0.0 0.0 0.0)) (`self.Aiming?`) (`self.AlwaysAimAtMouse`)) :`false` (`KismetMathLibrary.MakeRotator` 0.0 0.0 _returnvalue_yaw_2) :`true` (`KismetMathLibrary.MakeRotator` 0.0 0.0 _returnvalue_yaw)) false false))

(fn `UpdateMovementSpeed`
  (if (`self.Aiming?`)
    (set `CharacterMovementComponent.MaxWalkSpeed` (`self.AimingSpeed`) (`self.CharacterMovement`))
    (elif (`self.Sprinting`)
      (set `CharacterMovementComponent.MaxWalkSpeed` (`self.SprintSpeed`) (`self.CharacterMovement`))
      (else
        (set `CharacterMovementComponent.MaxWalkSpeed` (`self.WalkSpeed`) (`self.CharacterMovement`))))))

(fn `UserConstructionScript`
  (`SceneComponent.K2_SetWorldRotation` (`self.SpringArm`) (`KismetMathLibrary.MakeRotator` 0.0 -60.0 (+ (`self.CameraAngle`) 90.0)) false false))