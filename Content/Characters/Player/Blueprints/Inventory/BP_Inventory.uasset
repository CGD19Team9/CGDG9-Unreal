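; Player inventory Blueprint that handles pickups and keeps ammo counts per ammo type.
; AddToInventory switches on pickup type, but only ammo is stored; weapon and powerup pickups just print a debug message.
; AddAmmo, RemoveAmmo and GetAmmo work on the AmmoInventory map, with missing types reading as zero.
; RemoveAmmo only requires a count of at least one before subtracting, so totals can go negative.
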(event `AddToInventory`
  (params (PickupType :type "/Game/Characters/Player/Blueprints/Inventory/PickupType Enum" :default "NewEnumerator0") (AmmoType :type "/Game/Characters/Player/Blueprints/Inventory/AmmoType Enum" :default "NewEnumerator0") (Count :type Integer))
  (switch `/Game/Characters/Player/Blueprints/Inventory/PickupType` PickupType
    (:`NewEnumerator0`
      (`KismetSystemLibrary.PrintString` "PickedupWeapon"))
    (:`NewEnumerator1`
      (`KismetSystemLibrary.PrintString` "PickedupPowerup"))
    (:`NewEnumerator2`
      (`KismetSystemLibrary.PrintString` "PickedupAmmo")
      (`self.AddAmmo` AmmoType Count))))

(fn `AddAmmo`
  (params (AmmoType :type "/Game/Characters/Player/Blueprints/Inventory/AmmoType Enum" :default "NewEnumerator0") (Count :type Integer))
  (bind _ammoinventory (`self.AmmoInventory`))
  (bind (_value _returnvalue) (`BlueprintMapLibrary.Map_Find` _ammoinventory AmmoType))
  (if _returnvalue
    (`BlueprintMapLibrary.Map_Add` _ammoinventory AmmoType (+ _value Count))
    (else
      (`BlueprintMapLibrary.Map_Add` _ammoinventory AmmoType Count)))
  (`KismetSystemLibrary.PrintString` (`KismetStringLibrary.Concat_StrStr` (`|GetEnumeratorNameAsString` AmmoType) ": " (`KismetStringLibrary.Conv_IntToString` _value))))

(fn `GetAmmo`
  (params (AmmoType :type "/Game/Characters/Player/Blueprints/Inventory/AmmoType Enum" :default "NewEnumerator0"))
  (returns (Count :type Integer))
  (bind (_value _returnvalue) (`BlueprintMapLibrary.Map_Find` (`self.AmmoInventory`) AmmoType))
  (if _returnvalue
    (return _value)
    (else
      (return 0))))

(fn `RemoveAmmo`
  (params (AmmoType :type "/Game/Characters/Player/Blueprints/Inventory/AmmoType Enum" :default "NewEnumerator0") (Count :type Integer))
  (bind (_value _returnvalue) (`BlueprintMapLibrary.Map_Find` (`self.AmmoInventory`) AmmoType))
  (if (and _returnvalue (>= _value 1))
    (`BlueprintMapLibrary.Map_Add` (`self.AmmoInventory`) AmmoType (- _value Count))
    (`KismetSystemLibrary.PrintString` (`KismetStringLibrary.Concat_StrStr` "Removed ammo '" (`|GetEnumeratorNameAsString` AmmoType) "' Value = " (`KismetStringLibrary.Conv_IntToString` _value)))))