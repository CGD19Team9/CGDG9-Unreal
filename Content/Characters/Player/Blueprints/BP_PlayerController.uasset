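; Player controller that turns mouse, keyboard and action input into interface messages for the player character, covering movement, sprint, aiming, firing, reloading, weapon scrolling and interaction.
; Mouse movement traces under the visible cursor and writes the hit location, UI reference and controller onto BP_PlayerCharacter.
; Movement, sprint and rolls are gated by CanMove, with directional double-taps detected by delay-reset press counters triggering combat rolls.
; An older interaction popup and a restart call are left unconnected.
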(event `InputAction|Interact`
  (params (Key :type "Key Structure"))
  ;[1 1 1] Interact
  (:`Pressed`
    (if (`KismetSystemLibrary.IsValid` (`self.InteractionTarget`))
      (message `/Game/Characters/Player/Blueprints/BP_Interaction.Interact` (`self.InteractionTarget`) (`GameplayStatics.GetPlayerPawn` 0)))))

(event `self.ReceiveBeginPlay`
  ;[1 1 1] Setup
  (set `self.bShowMouseCursor` true))

(event `InputAxisKey|MouseX`
  (params (AxisValue :type "Float (single-precision)"))
  (bind (_bblockinghit _binitialoverlap _time _distance _location) (`GameplayStatics.BreakHitResult` (`self.GetHitResultUnderCursorByChannel` "TraceTypeQuery1")))
  ;[1 1 1] Update Mouse Location
  (if _bblockinghit :!label _label
    (bind _asbp_player_character (cast `/Game/Characters/Player/Blueprints/BP_PlayerCharacter` (`GameplayStatics.GetPlayerCharacter` 0)))
    (set `/Game/Characters/Player/Blueprints/BP_PlayerCharacter.UI_Widget` (`self.UIRef`) _asbp_player_character)
    (set `/Game/Characters/Player/Blueprints/BP_PlayerCharacter.PlayerController` self _asbp_player_character)
    (set `/Game/Characters/Player/Blueprints/BP_PlayerCharacter.MouseLocation` _location _asbp_player_character)))

(event `InputAction|Restart`
  (params (Key :type "Key Structure")))

(event `InputAxisKey|MouseY`
  (params (AxisValue :type "Float (single-precision)"))
  ;[1 1 1] Update Mouse Location
  (goto _label))

(event `InputAction|Aiming`
  (params (Key :type "Key Structure"))
  ;[1 1 1] Aiming
  (:`Pressed`
    (message `/Game/Characters/Player/Blueprints/CharacterControllerInterface.Aiming` (`GameplayStatics.GetPlayerCharacter` 0) true))
  (:`Released`
    (message `/Game/Characters/Player/Blueprints/CharacterControllerInterface.Aiming` (`GameplayStatics.GetPlayerCharacter` 0) false)))

(event `InputAxis|MoveRight`
  (params (AxisValue :type "Float (single-precision)"))
  ;[1 1 1] Walking
  (if (`self.canMove?`)
    (message `/Game/Characters/Player/Blueprints/CharacterControllerInterface.MoveRight` (`GameplayStatics.GetPlayerCharacter` 0) AxisValue)))

(event `InputAxis|MoveUp`
  (params (AxisValue :type "Float (single-precision)"))
  ;[1 1 1] Walking
  (if (`self.canMove?`)
    (message `/Game/Characters/Player/Blueprints/CharacterControllerInterface.MoveUp` (`GameplayStatics.GetPlayerCharacter` 0) AxisValue)))

(event `InputAction|Sprint`
  (params (Key :type "Key Structure"))
  ;[1 1 1] Sprint
  (:`Pressed`
    (if (`self.canMove?`)
      (message `/Game/Characters/Player/Blueprints/CharacterControllerInterface.Sprint` (`GameplayStatics.GetPlayerCharacter` 0) true)))
  (:`Released`
    (if (`self.canMove?`)
      (message `/Game/Characters/Player/Blueprints/CharacterControllerInterface.Sprint` (`GameplayStatics.GetPlayerCharacter` 0) false))))

(event `InputAction|RollFront`
  (params (Key :type "Key Structure"))
  ;[1 1 1] Rolling
  (:`Pressed`
    (if (`self.canMove?`)
      (bind _result (`/Engine/EditorBlueprintResources/StandardMacros.IncrementInt` (`self.FrontPresses`))
        (:`  `
          (if (> _result 1)
            (message `/Game/Characters/Player/Blueprints/CharacterControllerInterface.CombatRoll` (`GameplayStatics.GetPlayerCharacter` 0) "NewEnumerator0"))))))
  (:`Released`
    (`KismetSystemLibrary.Delay` (`self.DoubleTapPeriod`))
    (set `self.FrontPresses` 0)))

(event `InputAction|RollLeft`
  (params (Key :type "Key Structure"))
  ;[1 1 1] Rolling
  (:`Pressed`
    (if (`self.canMove?`)
      (bind _result (`/Engine/EditorBlueprintResources/StandardMacros.IncrementInt` (`self.LeftPresses`))
        (:`  `
          (if (> _result 1)
            (message `/Game/Characters/Player/Blueprints/CharacterControllerInterface.CombatRoll` (`GameplayStatics.GetPlayerCharacter` 0) "NewEnumerator2"))))))
  (:`Released`
    (`KismetSystemLibrary.Delay` (`self.DoubleTapPeriod`))
    (set `self.LeftPresses` 0)))

(event `InputAction|Fire`
  (params (Key :type "Key Structure"))
  ;[1 1 1] Fire
  (:`Pressed`
    (message `/Game/Characters/Player/Blueprints/CharacterControllerInterface.FireGun` (`GameplayStatics.GetPlayerCharacter` 0))))

(event `InputAction|RollBack`
  (params (Key :type "Key Structure"))
  ;[1 1 1] Rolling
  (:`Pressed`
    (if (`self.canMove?`)
      (bind _result (`/Engine/EditorBlueprintResources/StandardMacros.IncrementInt` (`self.BackPresses`))
        (:`  `
          (if (> _result 1)
            (message `/Game/Characters/Player/Blueprints/CharacterControllerInterface.CombatRoll` (`GameplayStatics.GetPlayerCharacter` 0) "NewEnumerator1"))))))
  (:`Released`
    (`KismetSystemLibrary.Delay` (`self.DoubleTapPeriod`))
    (set `self.BackPresses` 0)))

(event `InputAction|Reload`
  (params (Key :type "Key Structure"))
  ;[1 1 1] Reload
  (:`Pressed`
    (message `/Game/Characters/Player/Blueprints/CharacterControllerInterface.InterfaceReload` (`GameplayStatics.GetPlayerCharacter` 0))))

(event `InputAction|ScrollUp`
  (params (Key :type "Key Structure"))
  ;[1 1 1] Weapon Scrolling
  (:`Pressed`
    (message `/Game/Characters/Player/Blueprints/CharacterControllerInterface.WeaponScrollUp` (`GameplayStatics.GetPlayerCharacter` 0))))

(event `InputAction|RollRight`
  (params (Key :type "Key Structure"))
  ;[1 1 1] Rolling
  (:`Pressed`
    (if (`self.canMove?`)
      (bind _result (`/Engine/EditorBlueprintResources/StandardMacros.IncrementInt` (`self.RightPresses`))
        (:`  `
          (if (> _result 1)
            (message `/Game/Characters/Player/Blueprints/CharacterControllerInterface.CombatRoll` (`GameplayStatics.GetPlayerCharacter` 0) "NewEnumerator3"))))))
  (:`Released`
    (`KismetSystemLibrary.Delay` (`self.DoubleTapPeriod`))
    (set `self.RightPresses` 0)))

(event `InputAction|ScrollDown`
  (params (Key :type "Key Structure"))
  ;[1 1 1] Weapon Scrolling
  (:`Pressed`
    (message `/Game/Characters/Player/Blueprints/CharacterControllerInterface.WeaponScrollDown` (`GameplayStatics.GetPlayerCharacter` 0))))

(fn `UserConstructionScript`)